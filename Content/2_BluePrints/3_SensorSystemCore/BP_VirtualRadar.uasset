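; BP_VirtualRadar is a simulated radar sensor that finds the nearest obstacle around the actor.
; On BeginPlay it applies its RadarConfig.
; Each Tick it casts Visibility line traces along the configured bearings in the actor's local horizontal plane, ignoring the player pawn.
; The closest hit's distance and bearing are written to RadarData, which retains its last reading when no trace hits within range.
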(event EventBeginPlay
  (bind _radarconfig (Variables|Default|GetRadarConfig))
  ;[1 1 1] Default configure
  (Class|RadarSensorActor|Configure _radarconfig)
  (Variables|Default|SetTempDistance (.TraceLength (Utilities|Struct|BreakRadarConfig _radarconfig))))

(event EventTick
  (params (DeltaSeconds :type Float%20%28single-precision%29))
  (bind _self self)
  (bind _radarconfig (Variables|Default|GetRadarConfig))
  (bind (_fov _tracelength _tracenumber _tracebearings) (Utilities|Struct|BreakRadarConfig _radarconfig))
  (bind _returnvalue (Transformation|GetActorLocation _self))
  ;[1 1 1] Detect the minimum distance to obstacles and record its bearing
  (for _array_element _tracebearings
    (bind (_outhit _returnvalue_2) (Collision|LineTraceByChannel _returnvalue (+ _returnvalue (Math|Vector|RotateVector (Math|Vector|MakeVector (* (Math|Trig|Cos(Degrees) _array_element) _tracelength) (* (Math|Trig|Sin(Degrees) _array_element) _tracelength) 0.0) (Transformation|GetActorRotation _self))) "TraceTypeQuery1" false (Utilities|Array|MakeArray (Game|Player|GetPlayerPawn 0)) "None" true "(R=1.000000,G=0.000000,B=0.000000,A=1.000000)" "(R=0.000000,G=1.000000,B=0.000000,A=1.000000)" 0.2))
    (if _returnvalue_2
      (if (< (.Distance (Collision|BreakHitResult _outhit)) (Variables|Default|GetTempDistance))
        (Variables|Default|SetTempDistance (.Distance (Collision|BreakHitResult _outhit)))
        (Variables|Default|SetRadarData (Utilities|Struct|MakeRadarData (.Distance (Collision|BreakHitResult _outhit)) _array_element)))))
  (Variables|Default|SetTempDistance _tracelength))

(fn ConstructionScript)