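; BP_CheckPointManager is a one-shot checkpoint that marks task completion and records a player respawn point in GM_TruckOperation.
; An Enable flag, set on BeginPlay, lets only the first overlap of CheckPointGate fire, with no check on the overlapping actor.
; That overlap sets the game mode's TaskCompleteFlag and stores the checkpoint's own location and rotation as PlayerSpawnTransform, with Z forced to zero and unit scale.
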(event OnComponentBeginOverlap(CheckPointGate)
  (params (OverlappedComponent :type Primitive%20Component%20Object%20Reference) (OtherActor :type Actor%20Object%20Reference) (OtherComp :type Primitive%20Component%20Object%20Reference) (OtherBodyIndex :type Integer) (bFromSweep :type Boolean) (SweepResult :type Hit%20Result%20Structure%20%28by%20ref%29))
  (bind _returnvalue (Transformation|GetActorTransform))
  (bind (_location _rotation) (Math|Transform|BreakTransform _returnvalue))
  (bind (_x _y) (Math|Vector|BreakVector _location))
  (if (Variables|Default|GetEnable)
    (Variables|Default|SetEnable false)
    (bind _asgm_truck_operation (Utilities|Casting|CastToGM_TruckOperation (Game|GetGameMode)))
    (Variables|/Game/2_BluePrints/0_GameSystemCore/GM_TruckOperation.GM_TruckOperation_C|SetTaskCompleteFlag _asgm_truck_operation true)
    (Development|PrintString "Check point passed!")
    (Variables|/Script/HRVREP.GenericExperimentGameMode|SetPlayerSpawnTransform _asgm_truck_operation (Math|Transform|MakeTransform (Math|Vector|MakeVector _x _y 0.0) _rotation))
    (Development|PrintString "Check Point Location Recored!")))

(event EventBeginPlay
  (Variables|Default|SetEnable true))

(event Collision|EventActorBeginOverlap
  (params (OtherActor :type Actor%20Object%20Reference)))

(event EventTick
  (params (DeltaSeconds :type Float%20%28single-precision%29)))

(fn ConstructionScript)