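; BP_DataLogger is a data logger that accumulates text in a string and saves it to a file.
; LogData appends to DataString, and SaveFile passes it to SaveStringText with the directory and file name set through setters.
; A debug mode, switched off on BeginPlay, targets test.csv in the project Saved directory and uses keys 1 and 2 to test logging and saving.
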(event EventBeginPlay
  ;[1 1 1] Set Debug Mode
  (Variables|Default|SetDebug false)
  (if (Variables|Default|GetDebug)
    (CallFunction|SetDirectory (Class|KismetSystemLibrary|GetProjectSavedDirectory))
    (CallFunction|SetFileName "test.csv")))

(event EventTick
  (params (DeltaSeconds :type Float%20%28single-precision%29)))

(event Input|KeyboardEvents|1
  (params (Key :type Key%20Structure))
  (:Pressed
    (if (Variables|Default|GetDebug)
      (CallFunction|LogData (Utilities|String|Append (Utilities|String|ToString(Integer) (Class|KismetMathLibrary|GetSecond (Math|DateTime|UTCNow))) " 
 "))
      (Development|PrintString (Variables|Default|GetDataString)))))

(event Input|KeyboardEvents|2
  (params (Key :type Key%20Structure))
  (:Pressed
    (if (Variables|Default|GetDebug)
      (bind _flag (CallFunction|SaveFile))
      (if _flag
        (Development|PrintString "Data Saved")
        (else
          (Development|PrintString "Fail: Data Saving"))))))

(fn ConstructionScript)

(fn SetDirectory
  (params (Directory :type String))
  (Variables|Default|SetDirectory Directory))

(fn SetFileName
  (params (FileName :type String))
  (Variables|Default|SetFileName FileName))

(fn SaveFile
  (bind _returnvalue (Class|CSVFileManager|SaveStringText (Variables|Default|GetDirectory) (Variables|Default|GetFileName) (Variables|Default|GetDataString) false))
  (return _returnvalue))

(fn LogData
  (params (NewString :type String))
  (Variables|Default|SetDataString (Utilities|String|Append (Variables|Default|GetDataString) NewString)))