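; BP_DataLoggerSystem is a key-driven test harness for logging timestamps to a CSV file through a DataLoggerManager object.
; BeginPlay constructs the manager and targets InEngineData.csv in the project's Saved directory with a two-column time header.
; N logs the current UTC timestamp in both columns; M saves the log and prints the result.
; Despite its name, GetFrameTime builds a wall-clock date-time string to the millisecond, without separating day from hour.
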(event EventBeginPlay
  (bind _returnvalue (Game|ConstructObjectfromClass "/Script/HRVREP.DataLoggerManager"))
  (bind _output_get (Variables|Default|SetDataLogger _returnvalue))
  (Class|DataLoggerManager|SetDirectory _output_get (Class|KismetSystemLibrary|GetProjectSavedDirectory))
  (Class|DataLoggerManager|SetFileName _output_get "InEngineData.csv")
  (Class|DataLoggerManager|SetDataHeader _output_get "Time,Time"))

(event Collision|EventActorBeginOverlap
  (params (OtherActor :type Actor%20Object%20Reference)))

(event EventTick
  (params (DeltaSeconds :type Float%20%28single-precision%29)))

(event Input|KeyboardEvents|N
  (params (Key :type Key%20Structure))
  (:Pressed
    (bind _timenow (CallFunction|GetFrameTime))
    (Class|DataLoggerManager|LogNewData (Variables|Default|GetDataLogger) (Utilities|String|Append _timenow "," _timenow))))

(event Input|KeyboardEvents|M
  (params (Key :type Key%20Structure))
  (:Pressed
    (bind _returnvalue (Class|DataLoggerManager|SaveLog (Variables|Default|GetDataLogger)))
    (if _returnvalue
      (Development|PrintString "Data Saved")
      (else
        (Development|PrintString "Fail: Data Saving")))))

(fn ConstructionScript)

(fn GetFrameTime
  (bind _returnvalue (Math|DateTime|UTCNow))
  (return (Utilities|String|Append (Utilities|String|ToString(Integer) (Class|KismetMathLibrary|GetYear _returnvalue)) "-" (Utilities|String|ToString(Integer) (Class|KismetMathLibrary|GetMonth _returnvalue)) "-" (Utilities|String|ToString(Integer) (Class|KismetMathLibrary|GetDay _returnvalue)) " " (Utilities|String|ToString(Integer) (Class|KismetMathLibrary|GetHour _returnvalue)) ":" (Utilities|String|ToString(Integer) (Class|KismetMathLibrary|GetMinute _returnvalue)) ":" (Utilities|String|ToString(Integer) (Class|KismetMathLibrary|GetSecond _returnvalue)) ":" (Utilities|String|ToString(Integer) (Math|DateTime|GetMillisecond _returnvalue)))))