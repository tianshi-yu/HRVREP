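; Drivable truck pawn whose Enhanced Input actions feed the vehicle movement component, with brake lights following brake input.
; It toggles between inside and outside cameras, with mouse look and a movable, resettable driver viewpoint.
; Tick updates the truck sensor readings and turns the steering wheel from the first wheel's steer angle.
; It adds a temporary driving HUD and a Delete-key menu; GearUp lowers the gear number and GearDown raises it.
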(event Input|EnhancedActionEvents|EnhancedInputActionIA_Throttle
  (params (ActionValue :type Float%20%28double-precision%29) (ElapsedSeconds :type Float%20%28double-precision%29) (TriggeredSeconds :type Float%20%28double-precision%29) (InputAction :type Input%20Action%20Object%20Reference :default "/Game/2_BluePrints/2_AvatarSystemCore/EnhancedInput/Driving_Keys/IA_Throttle.IA_Throttle"))
  ;[1 1 1] Vehicle Movement Control
  (:Triggered
    (Class|ChaosVehicleMovementComponent|SetThrottleInput (Variables|Default|GetVehicleMovementComponent) ActionValue :!label _label))
  (:Started
    (goto _label))
  (:Ongoing
    (goto _label))
  (:Canceled
    (goto _label))
  (:Completed
    (goto _label)))

(event Input|EnhancedActionEvents|EnhancedInputActionIA_Brake
  (params (ActionValue :type Float%20%28double-precision%29) (ElapsedSeconds :type Float%20%28double-precision%29) (TriggeredSeconds :type Float%20%28double-precision%29) (InputAction :type Input%20Action%20Object%20Reference :default "/Game/2_BluePrints/2_AvatarSystemCore/EnhancedInput/Driving_Keys/IA_Brake.IA_Brake"))
  ;[1 1 1] Vehicle Movement Control
  (:Triggered
    (Class|ChaosVehicleMovementComponent|SetBrakeInput (Variables|Default|GetVehicleMovementComponent) ActionValue :!label _label)
    ;;[1 1 1] Brake Lights
    (CallFunction|ToggleBrakeLight (> ActionValue 0.0)))
  (:Started
    (goto _label))
  (:Ongoing
    (goto _label))
  (:Canceled
    (goto _label))
  (:Completed
    (goto _label)))

(event Input|EnhancedActionEvents|EnhancedInputActionIA_DriverCameraRight
  (params (ActionValue :type Boolean) (ElapsedSeconds :type Float%20%28double-precision%29) (TriggeredSeconds :type Float%20%28double-precision%29) (InputAction :type Input%20Action%20Object%20Reference :default "/Game/2_BluePrints/2_AvatarSystemCore/EnhancedInput/Driving_Keys/IA_DriverCameraRight.IA_DriverCameraRight"))
  (bind _insidecameraroot (Variables|Default|GetInsideCameraRoot))
  ;[1 1 1] Camera Control
  (:Triggered
    (Transformation|AddWorldOffset _insidecameraroot (* (Variables|Default|GetDriverMovementSpeed) (Math|Vector|GetRightVector _insidecameraroot)) false true :!label _label))
  (:Ongoing
    (goto _label)))

(event Input|EnhancedActionEvents|EnhancedInputActionIA_GearDown
  (params (ActionValue :type Boolean) (ElapsedSeconds :type Float%20%28double-precision%29) (TriggeredSeconds :type Float%20%28double-precision%29) (InputAction :type Input%20Action%20Object%20Reference :default "/Game/2_BluePrints/2_AvatarSystemCore/EnhancedInput/Driving_Keys/IA_GearDown.IA_GearDown"))
  (bind _vehiclemovementcomponent (Variables|Default|GetVehicleMovementComponent))
  ;[1 1 1] Vehicle Movement Control
  (:Ongoing
    (Class|ChaosVehicleMovementComponent|SetTargetGear _vehiclemovementcomponent (+ (Class|ChaosVehicleMovementComponent|GetCurrentGear _vehiclemovementcomponent) 1) true :!label _label))
  (:Completed
    (goto _label)))

(event Input|EnhancedActionEvents|EnhancedInputActionIA_SwitchManualAuto
  (params (ActionValue :type Boolean) (ElapsedSeconds :type Float%20%28double-precision%29) (TriggeredSeconds :type Float%20%28double-precision%29) (InputAction :type Input%20Action%20Object%20Reference :default "/Game/2_BluePrints/2_AvatarSystemCore/EnhancedInput/Driving_Keys/IA_SwitchManualAuto.IA_SwitchManualAuto"))
  (bind _vehiclemovementcomponent (Variables|Default|GetVehicleMovementComponent))
  ;[1 1 1] Comment
  (:Completed
    (Class|ChaosVehicleMovementComponent|SetUseAutomaticGears _vehiclemovementcomponent (not (Class|ChaosVehicleMovementComponent|GetUseAutoGears _vehiclemovementcomponent)))))

(event Input|EnhancedActionEvents|EnhancedInputActionIA_Steering
  (params (ActionValue :type Float%20%28double-precision%29) (ElapsedSeconds :type Float%20%28double-precision%29) (TriggeredSeconds :type Float%20%28double-precision%29) (InputAction :type Input%20Action%20Object%20Reference :default "/Game/2_BluePrints/2_AvatarSystemCore/EnhancedInput/Driving_Keys/IA_Steering.IA_Steering"))
  ;[1 1 1] Vehicle Movement Control
  (:Triggered
    (Class|ChaosVehicleMovementComponent|SetSteeringInput (Variables|Default|GetVehicleMovementComponent) ActionValue :!label _label))
  (:Started
    (goto _label))
  (:Ongoing
    (goto _label))
  (:Canceled
    (goto _label))
  (:Completed
    (goto _label)))

(event Input|EnhancedActionEvents|EnhancedInputActionIA_Handbrake
  (params (ActionValue :type Boolean) (ElapsedSeconds :type Float%20%28double-precision%29) (TriggeredSeconds :type Float%20%28double-precision%29) (InputAction :type Input%20Action%20Object%20Reference :default "/Game/2_BluePrints/2_AvatarSystemCore/EnhancedInput/Driving_Keys/IA_Handbrake.IA_Handbrake"))
  ;[1 1 1] Vehicle Movement Control
  (:Triggered
    (Class|ChaosVehicleMovementComponent|SetHandbrakeInput (Variables|Default|GetVehicleMovementComponent) ActionValue :!label _label))
  (:Started
    (goto _label))
  (:Ongoing
    (goto _label))
  (:Canceled
    (goto _label))
  (:Completed
    (goto _label)))

(event Input|EnhancedActionEvents|EnhancedInputActionIA_ChangeDriveView
  (params (ActionValue :type Boolean) (ElapsedSeconds :type Float%20%28double-precision%29) (TriggeredSeconds :type Float%20%28double-precision%29) (InputAction :type Input%20Action%20Object%20Reference :default "/Game/2_BluePrints/2_AvatarSystemCore/EnhancedInput/Driving_Keys/IA_ChangeDriveView.IA_ChangeDriveView"))
  ;[1 1 1] Camera Switch
  (:Completed
    (Utilities|FlowControl|FlipFlop
      (:A
        (Components|Activation|SetActive (Variables|Default|GetInside%20Camera) false false)
        (Components|Activation|SetActive (Variables|Default|GetOutside%20Camera) true false))
      (:B
        (Components|Activation|SetActive (Variables|Default|GetInside%20Camera) true false)
        (Components|Activation|SetActive (Variables|Default|GetOutside%20Camera) false false)))))

(event Input|EnhancedActionEvents|EnhancedInputActionIA_GearUp
  (params (ActionValue :type Boolean) (ElapsedSeconds :type Float%20%28double-precision%29) (TriggeredSeconds :type Float%20%28double-precision%29) (InputAction :type Input%20Action%20Object%20Reference :default "/Game/2_BluePrints/2_AvatarSystemCore/EnhancedInput/Driving_Keys/IA_GearUp.IA_GearUp"))
  (bind _vehiclemovementcomponent (Variables|Default|GetVehicleMovementComponent))
  ;[1 1 1] Vehicle Movement Control
  (:Ongoing
    (Class|ChaosVehicleMovementComponent|SetTargetGear _vehiclemovementcomponent (- (Class|ChaosVehicleMovementComponent|GetCurrentGear _vehiclemovementcomponent) 1) true :!label _label))
  (:Completed
    (goto _label)))

(event Input|EnhancedActionEvents|EnhancedInputActionIA_DriverCameraReset
  (params (ActionValue :type Boolean) (ElapsedSeconds :type Float%20%28double-precision%29) (TriggeredSeconds :type Float%20%28double-precision%29) (InputAction :type Input%20Action%20Object%20Reference :default "/Game/2_BluePrints/2_AvatarSystemCore/EnhancedInput/Driving_Keys/IA_DriverCameraReset.IA_DriverCameraReset"))
  ;[1 1 1] Camera Control
  (Transformation|SetRelativeTransform (Variables|Default|GetInsideCameraRoot) (Variables|Default|GetOriginalInsideCameraTransform) false true))

(event Input|EnhancedActionEvents|EnhancedInputActionIA_DriverCameraForward
  (params (ActionValue :type Boolean) (ElapsedSeconds :type Float%20%28double-precision%29) (TriggeredSeconds :type Float%20%28double-precision%29) (InputAction :type Input%20Action%20Object%20Reference :default "/Game/2_BluePrints/2_AvatarSystemCore/EnhancedInput/Driving_Keys/IA_DriverCameraForward.IA_DriverCameraForward"))
  (bind _insidecameraroot (Variables|Default|GetInsideCameraRoot))
  ;[1 1 1] Camera Control
  (:Triggered
    (Transformation|AddWorldOffset _insidecameraroot (* (Variables|Default|GetDriverMovementSpeed) (Math|Vector|GetForwardVector _insidecameraroot)) false true :!label _label))
  (:Ongoing
    (goto _label)))

(event Input|EnhancedActionEvents|EnhancedInputActionIA_DriverCameraBackward
  (params (ActionValue :type Boolean) (ElapsedSeconds :type Float%20%28double-precision%29) (TriggeredSeconds :type Float%20%28double-precision%29) (InputAction :type Input%20Action%20Object%20Reference :default "/Game/2_BluePrints/2_AvatarSystemCore/EnhancedInput/Driving_Keys/IA_DriverCameraBackward.IA_DriverCameraBackward"))
  (bind _insidecameraroot (Variables|Default|GetInsideCameraRoot))
  ;[1 1 1] Camera Control
  (:Triggered
    (Transformation|AddWorldOffset _insidecameraroot (* (Variables|Default|GetDriverMovementSpeed) (Math|Vector|NegateVector (Math|Vector|GetForwardVector _insidecameraroot))) false true :!label _label))
  (:Ongoing
    (goto _label)))

(event Input|EnhancedActionEvents|EnhancedInputActionIA_DriverCameraLeft
  (params (ActionValue :type Boolean) (ElapsedSeconds :type Float%20%28double-precision%29) (TriggeredSeconds :type Float%20%28double-precision%29) (InputAction :type Input%20Action%20Object%20Reference :default "/Game/2_BluePrints/2_AvatarSystemCore/EnhancedInput/Driving_Keys/IA_DriverCameraLeft.IA_DriverCameraLeft"))
  (bind _insidecameraroot (Variables|Default|GetInsideCameraRoot))
  ;[1 1 1] Camera Control
  (:Triggered
    (Transformation|AddWorldOffset _insidecameraroot (* (Variables|Default|GetDriverMovementSpeed) (Math|Vector|NegateVector (Math|Vector|GetRightVector _insidecameraroot))) false true :!label _label))
  (:Ongoing
    (goto _label)))

(event EventBeginPlay
  ;[1 1 1] Initialisation
  (Utilities|FlowControl|Sequence
    (:then_0
      ;;[1 1 1] Add HUD - Temporary
      (bind _returnvalue (UserInterface|CreateWidget "/Game/2_BluePrints/5_UISystemCore/WBP_DrivingHUD.WBP_DrivingHUD_C"))
      (UserInterface|Viewport|AddtoViewport _returnvalue 0))
    (:then_1
      ;;[1 1 1] Config enhanced input system
      (bind _asplayer_controller (Utilities|Casting|CastToPlayerController (Pawn|GetController)))
      (Input|AddMappingContext (PlayerController|LocalPlayerSubsystems|GetEnhancedInputLocalPlayerSubsystem _asplayer_controller) "/Game/2_BluePrints/2_AvatarSystemCore/EnhancedInput/IMC_DrivingInputs.IMC_DrivingInputs" 0 "(bIgnoreAllPressedKeysUntilRelease=True,bForceImmediately=False,bNotifyUserSettings=False)"))
    (:then_2
      ;;[1 1 1] Camera settings
      (Variables|Default|SetOriginalInsideCameraTransform (Transformation|GetRelativeTransform (Variables|Default|GetInsideCameraRoot)))
      (Variables|Default|SetOriginalOutsideCameraTransform (Transformation|GetRelativeTransform (Variables|Default|GetOutsideCameraSpringArm)))
      (Variables|Default|SetDriverMovementSpeed "1.250000,1.250000,0.000000"))))

(event EventTick
  (params (DeltaSeconds :type Float%20%28single-precision%29))
  (bind _vehiclemovementcomponent (Variables|Default|GetVehicleMovementComponent))
  ;[1 1 1] Tick update
  (Utilities|FlowControl|Sequence
    (:then_0
      ;;[1 1 1] Update Sensor Readings
      (Class|TruckPawnSensorManager|UpdateReadings (Variables|Default|GetTrcukPawnSensor)))
    (:then_1
      ;;[1 1 1] Steering Animation
      (bind _aschaos_wheeled_vehicle_movement_component (Utilities|Casting|CastToChaosWheeledVehicleMovementComponent _vehiclemovementcomponent))
      (Class|ChaosVehicleMovementComponent|GetSteeringInput _vehiclemovementcomponent)
      (Transformation|SetRelativeRotation (Variables|Default|GetSteeringWheel) (Math|Rotator|MakeRotator (* 5.0 (Class|ChaosVehicleWheel|GetSteerAngle (Utilities|Array|Get(acopy) (Variables|/Script/ChaosVehicles.ChaosWheeledVehicleMovementComponent|GetWheels _aschaos_wheeled_vehicle_movement_component)))) 0.0 0.0) false false))))

(event Input|MouseEvents|MouseX
  (params (AxisValue :type Float%20%28single-precision%29))
  ;[1 1 1] Camera Control
  (Transformation|AddRelativeRotation (Variables|Default|GetOutsideCameraSpringArm) (Math|Rotator|MakeRotator 0.0 0.0 AxisValue) false false))

(event Input|MouseEvents|MouseY
  (params (AxisValue :type Float%20%28single-precision%29))
  ;[1 1 1] Camera Control
  (Transformation|AddRelativeRotation (Variables|Default|GetOutsideCameraSpringArm) (Math|Rotator|MakeRotator 0.0 AxisValue 0.0) false false))

(event Input|KeyboardEvents|Delete
  (params (Key :type Key%20Structure :default "None"))
  (bind _returnvalue (Game|GetPlayerController 0))
  ;[1 1 1] Main Menu
  (:Pressed
    (Utilities|FlowControl|Sequence
      (:then_0
        (Utilities|FlowControl|DoOnce false
          (:Completed
            (bind _returnvalue_2 (UserInterface|CreateWidget "/Game/2_BluePrints/5_UISystemCore/WBP_MainMenu.WBP_MainMenu_C")))))
      (:then_1
        (Utilities|FlowControl|FlipFlop
          (:A
            (UserInterface|Viewport|AddtoViewport _returnvalue_2 0)
            (Input|SetInputModeGameandUI _returnvalue _returnvalue_2 "DoNotLock" true false))
          (:B
            (Input|SetInputModeGameOnly _returnvalue false)
            (Widget|RemovefromParent _returnvalue_2)))))))

(fn ConstructionScript)

(fn ToggleBrakeLight
  (params (On? :type Boolean))
  (Rendering|SetVisibility (Variables|Default|GetBrakeLight1) On? false))