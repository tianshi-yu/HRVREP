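; Game mode for a VR truck driving experiment, extending a parent training, task, iteration and session state flow with flag-driven completion checks.
; On start it enables supported DLSS and Reflex and registers truck, four radar and Vive XR headset sensors, plus a Delsys connection.
; Each task update logs all sensor readings to per-iteration files under the user's session directory.
; Task and iteration starts reset the truck to its spawn transform.
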(event EventBeginPlay
  (bind (_bissupported _optimalscreenpercentage _bisfixedscreenpercentage _minscreenpercentage _maxscreenpercentage) (Class|DLSSLibrary|GetDLSSModeInformation "UltraPerformance"))
  ;[1 1 1] Check DLSS Support
  (for _array_element (Class|DLSSLibrary|GetSupportedDLSSModes)
    (Development|PrintString (Utilities|String|Append (Utilities|String|MakeLiteralString "DLSS-SR Supported:") (Utilities|String|EnumtoString _array_element))))
  (Development|PrintString (Utilities|String|Append "DLSS: " (Utilities|String|ToString(Float) _optimalscreenpercentage) ", " (Utilities|String|ToString(Float) _minscreenpercentage) ", " (Utilities|String|ToString(Float) _maxscreenpercentage)))
  (Development|PrintString (Utilities|String|Append (Utilities|String|MakeLiteralString "DLSS-RR Supported:") (Utilities|String|EnumtoString (Class|DLSSLibrary|QueryDLSSRRSupport))))
  ;[1 1 1] DLSS SR (RR not supported yet)
  (Utilities|FlowControl|Sequence
    (:then_0
      (if (Class|DLSSLibrary|IsDLSSSupported)
        (Development|ExecuteConsoleCommand "r.NGX.Enable 1 -ngxenable" 0)
        (Development|ExecuteConsoleCommand "r.NGX.DLSS.Enable 1" 0)
        (Development|ExecuteConsoleCommand "r.ScreenPercentage 33.3" 0)
        (Class|DLSSLibrary|EnableDLSS true)
        (Development|PrintString (Utilities|String|Append (Utilities|String|MakeLiteralString "DLSS-SR Enabled:") (Utilities|String|ToString(Boolean) (Class|DLSSLibrary|IsDLSSEnabled))))))
    (:then_1
      (if (Class|DLSSLibrary|IsDLSSRRSupported)
        (Development|ExecuteConsoleCommand "r.NGX.DLSS.denoisermode 1" 0)
        (Development|ExecuteConsoleCommand "r.Lumen.Reflections.BilateralFilter 0" 0)
        (Development|ExecuteConsoleCommand "r.Lumen.Reflections.ScreenSpaceReconstruction 0" 0)
        (Development|ExecuteConsoleCommand "r.lumen.Reflections.Temporal 0" 0)
        (Development|ExecuteConsoleCommand "r.Shadow.Denoiser 0" 0)
        (Class|DLSSLibrary|EnableDLSSRR true)
        (Development|PrintString (Utilities|String|Append (Utilities|String|MakeLiteralString "DLSS-RR Enabled:") (Utilities|String|ToString(Boolean) (Class|DLSSLibrary|IsDLSSRREnabled))))))
    (:then_2
      (if (Class|StreamlineLibraryReflex|IsReflexSupported)
        (Class|StreamlineLibraryReflex|SetReflexMode "Enabled")
        (Development|PrintString (Utilities|String|Append (Utilities|String|MakeLiteralString "Reflex Eanble: ") (Utilities|String|EnumtoString (Class|StreamlineLibraryReflex|GetReflexMode))))))))

(event EventTick
  (params (DeltaSeconds :type Float%20%28single-precision%29))
  ;[1 1 1] Logic has been implemented in C++
  (Variables|Default|SetFrameDeltaSecond DeltaSeconds))

(event EventInitIteration
  ;[1 1 1] Handle Iteration Complete, create new iteration data logger
  (|CallParentFunction)
  (Variables|Default|SetPlayerSpawnTransform (Transformation|GetActorTransform (Class|GameModeBase|FindPlayerStart (Game|GetPlayerController 0))))
  (Utilities|EnableCheckPoints)
  (Utilities|ResetPawnTransform)
  (Utilities|AddinEngineDataLogger))

(event EventInitSession
  ;[1 1 1] Handle Session Complete
  (|CallParentFunction))

(event EventHandleTaskFail
  ;[1 1 1] Task fail
  (|CallParentFunction)
  (Development|PrintString "Task Failed!"))

(event EventInitTask
  ;[1 1 1] Task fail
  (|CallParentFunction)
  (Utilities|ResetPawnTransform)
  ;;[1 1 1] Avoid collision be triggered multiple times
  (Variables|Default|SetTaskFailFlag false)
  (Development|PrintString "Reset current task!"))

(event EventEndPlay
  (params (EndPlayReason :type EEndPlayReason%20Enum :default "Destroyed"))
  ;[1 1 1] End
  (Development|PrintString "End Experiment")
  (Utilities|CloseAllDataLogger)
  (Utilities|FlowControl|Delay 1.0)
  (Game|QuitGame 0 "Quit" false))

(event EventInitSystem
  (bind _returnvalue (Subsystems|GetUserSubSystem))
  (bind _radarconfig (Utilities|Struct|MakeRadarConfig 1.2e+02 2e+04 12))
  (bind _truckpawnsensormanager (Variables|Default|GetTruckPawnSensorManager))
  (bind _vivexrheadsetsensormanager (Variables|Default|GetViveXRHeadsetSensorManager))
  ;[1 1 1] Initialise the system
  (Utilities|FlowControl|Sequence
    (:then_0
      ;;[1 1 1] Set User information - Debug only
      (if (Variables|Default|GetDebug)
        (Class|UserSubSystem|SetUserData _returnvalue (Utilities|Struct|MakeGenericUserData "Test" "Bot" 1995 175))
        (Class|UserSubSystem|SetUserDirectory _returnvalue)
        (Class|UserSubSystem|SaveUserData _returnvalue)
        (Development|PrintString "Debug User Used")))
    (:then_1
      ;;[1 1 1] Sensors
      (Utilities|FlowControl|Sequence
        (:then_0
          (bind _asbp_vrtruck_pawn (Utilities|Casting|CastToBP_VRTruckPawn (Game|Player|GetPlayerPawn 0)))
          (bind _returnvalue_2 (Settings|GetGameUserSettings))
          (Class|TruckPawnSensorManager|InitTruckPawnSensor _truckpawnsensormanager (Utilities|String|MakeLiteralString "TruckPawn") (Class|GameUserSettings|GetFrameRateLimit _returnvalue_2) (Variables|/Script/ChaosVehicles.WheeledVehiclePawn|GetVehicleMovementComponent _asbp_vrtruck_pawn))
          (Class|SensorSubSystem|AddSensor (Subsystems|GetSensorSubSystem) _truckpawnsensormanager))
        (:then_1
          (bind _out (Default|GetRadars _asbp_vrtruck_pawn))
          (CallFunction|InitRadarSensorfromMap _out (Class|GameUserSettings|GetFrameRateLimit _returnvalue_2) (Utilities|String|MakeLiteralString "FrontRadar") (Variables|Default|GetFrontRadarSensorManager) _radarconfig)
          (CallFunction|InitRadarSensorfromMap _out (Class|GameUserSettings|GetFrameRateLimit _returnvalue_2) (Utilities|String|MakeLiteralString "RearRadar") (Variables|Default|GetRearRadarSensorManager) _radarconfig)
          (CallFunction|InitRadarSensorfromMap _out (Class|GameUserSettings|GetFrameRateLimit _returnvalue_2) (Utilities|String|MakeLiteralString "RightRadar") (Variables|Default|GetRightRadarSensorManager) _radarconfig)
          (CallFunction|InitRadarSensorfromMap _out (Class|GameUserSettings|GetFrameRateLimit _returnvalue_2) (Utilities|String|MakeLiteralString "LeftRadar") (Variables|Default|GetLeftRadarSensorManager) _radarconfig))
        (:then_2
          (Class|GenericSensorManager|InitSensor _vivexrheadsetsensormanager (Utilities|String|MakeLiteralString "ViveXR") (Class|GameUserSettings|GetFrameRateLimit _returnvalue_2))
          (Class|SensorSubSystem|AddSensor (Subsystems|GetSensorSubSystem) _vivexrheadsetsensormanager))
        (:then_3
          (Class|DelsysTrignoEMG|Connect (Variables|Default|GetDelsys)))))
    (:then_2
      ;;[1 1 1] Configure Data loggers
      (Utilities|FlowControl|DelayUntilNextTick)
      (Class|SensorSubSystem|UpdateAllReadings (Subsystems|GetSensorSubSystem))
      (Utilities|AddinEngineDataLogger))
    (:then_3
      ;;[1 1 1] Record initial spawn transform
      (Variables|Default|SetPlayerSpawnTransform (Transformation|GetActorTransform (Game|Player|GetPlayerPawn 0))))))

(event EventHandleTrainingComplete
  ;[1 1 1] Handle Training Process and Complete
  (|CallParentFunction)
  (Development|PrintString "Training Complete!"))

(event EventHandleTrainingProcess
  ;[1 1 1] Handle Training Process and Complete
  (|CallParentFunction))

(event EventHandleTaskProcess
  (bind _returnvalue (Subsystems|GetSensorSubSystem))
  ;[1 1 1] Handle Task Process and Complete
  (|CallParentFunction)
  (bind _returnvalue_2 (Class|Misc|GetTimeNow))
  (Class|SensorSubSystem|UpdateAllReadings _returnvalue)
  (bind _returnvalue_3 (Class|SensorSubSystem|RetrieveAllVarValuesStr _returnvalue ","))
  (Class|DataLoggerManager|LogNewData (Class|DataLoggerSubSystem|FindDataLoggerbyName (Subsystems|GetDataLoggerSubSystem) (.Value (Utilities|Map|Find (Variables|Default|GetDataLoggerName) "InEngineData"))) (Utilities|String|Append _returnvalue_2 "," (Utilities|String|ToString(Float) (Variables|Default|GetFrameDeltaSecond)) "," (Utilities|Array|Get(acopy) (Variables|Default|GetTaskList) (Variables|Default|GetTaskNumber)) "," (Utilities|String|ToString(Integer) (Variables|Default|GetTaskAttemptNumber)) "," _returnvalue_3)))

(event EventHandleTaskComplete
  ;[1 1 1] Handle Task Process and Complete
  (|CallParentFunction)
  (Development|PrintString "Task Compelte!"))

(event EventHandleIterationComplete
  ;[1 1 1] Handle Iteration Complete, create new iteration data logger
  (Utilities|CloseAllDataLogger)
  (|CallParentFunction)
  (Development|PrintString "Iteration Complete!"))

(event EventHandleSessionComplete
  ;[1 1 1] Handle Session Complete
  (|CallParentFunction)
  (Development|PrintString "Session Complete"))

(fn ConstructionScript)

(fn CheckTrainingComplete
  (if (Variables|Default|GetSkipCurrentState)
    (Variables|Default|SetSkipCurrentState false)
    (return true)
    (else
      (return false))))

(fn CheckTaskComplete
  (if (Variables|Default|GetTaskCompleteFlag)
    (Variables|Default|SetTaskCompleteFlag false)
    (return true)
    (elif (Variables|Default|GetSkipCurrentState)
      (Variables|Default|SetSkipCurrentState false)
      (return true)
      (else
        (return false)))))

(fn CheckIterationComplete
  (bind _outcomplete (|CallParentFunction))
  (return _outcomplete))

(fn CheckSessionComplete
  (bind _outcomplete (|CallParentFunction))
  (return _outcomplete))

(fn CheckExperimentComplete
  (bind _outcomplete (|CallParentFunction))
  (return _outcomplete))

(fn CheckTaskFail
  (if (Variables|Default|GetTaskFailFlag)
    (return true)
    (else
      (return false))))

(fn InitRadarSensorfromMap
  (params (RadarActorsMap :type Map%20of%20Strings%20to%20Objects) (InRate :type Float%20%28single-precision%29) (InName :type String) (TargetManager :type Radar%20Sensor%20Manager%20Object%20Reference) (RadarConfig :type Radar%20Config%20Structure))
  (Class|RadarSensorManager|InitRadarSensor TargetManager InName InRate (.Value (Utilities|Map|Find RadarActorsMap InName)) RadarConfig)
  (bind _returnvalue (Class|SensorSubSystem|AddSensor (Subsystems|GetSensorSubSystem) TargetManager))
  (return _returnvalue))