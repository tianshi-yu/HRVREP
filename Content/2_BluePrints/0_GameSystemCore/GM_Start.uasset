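; GM_Start is the startup game mode that opens the main menu and applies rendering settings when play begins.
; BeginPlay caps the frame rate, turns off VR stereo and adds WBP_MainMenu to the viewport.
; It then prints DLSS support and enables DLSS Super Resolution at a reduced screen percentage without gating on that result.
; A Ray Reconstruction setup that disables Lumen reflection and shadow denoisers is left unconnected and never runs.
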(event EventBeginPlay
  (Development|ExecuteConsoleCommand "t.MaxFps 60" 0)
  (Development|ExecuteConsoleCommand "vr.bEnableStereo False" 0)
  (bind _returnvalue (UserInterface|CreateWidget "/Game/2_BluePrints/5_UISystemCore/WBP_MainMenu.WBP_MainMenu_C"))
  (UserInterface|Viewport|AddtoViewport _returnvalue 0)
  (Development|PrintString (Utilities|String|Append (Utilities|String|MakeLiteralString "DLSS-SR Supported:") (Utilities|String|EnumtoString (Class|DLSSLibrary|QueryDLSSSupport)) " 
" (Utilities|String|MakeLiteralString "DLSS-RR Supported:") (Utilities|String|EnumtoString (Class|DLSSLibrary|QueryDLSSRRSupport))))
  (Utilities|FlowControl|Sequence
    (:then_0
      ;[1 1 1] DLSS SR (RR not supported yet)
      (Class|DLSSLibrary|EnableDLSS true)
      (Development|ExecuteConsoleCommand "r.NGX.Enable 1 -ngxenable" 0)
      (Development|ExecuteConsoleCommand "r.NGX.DLSS.Enable 1" 0)
      (Development|ExecuteConsoleCommand "r.ScreenPercentage 50" 0)
      (Development|PrintString (Utilities|String|Append (Utilities|String|MakeLiteralString "DLSS-SR Enabled:") (Utilities|String|ToString(Boolean) (Class|DLSSLibrary|IsDLSSEnabled)))))))

(event EventTick
  (params (DeltaSeconds :type Float%20%28single-precision%29)))

(fn ConstructionScript)