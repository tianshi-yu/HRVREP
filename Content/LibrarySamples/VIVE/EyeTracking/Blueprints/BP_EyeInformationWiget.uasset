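; VIVE eye tracking sample Blueprint that shows live per-eye tracking data on a widget.
; On BeginPlay it creates a WBP_EyeInformation widget and assigns it to its EyeWidget component.
; Every Tick it polls stereo gaze data and HTC gaze validity, pupil and eye geometric data.
; It writes each left and right value, from origin and direction to pupil size and openness, straight into the widget's text fields.
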(event EventBeginPlay
  (bind _returnvalue (UserInterface|CreateWidget "/Game/LibrarySamples/VIVE/EyeTracking/Blueprints/WBP_EyeInformation.WBP_EyeInformation_C"))
  (bind _output_get (Variables|Default|SetEyeInformationWidget _returnvalue))
  (UserInterface|SetWidget (Variables|Default|GetEyeWidget) _output_get))

(event EventTick
  (params (DeltaSeconds :type Float%20%28single-precision%29))
  (bind _returnvalue (Class|ViveOpenXREyeTrackerFunctionLibrary|GetHTCEyeGeometricData))
  (bind _returnvalue_2 (Class|ViveOpenXREyeTrackerFunctionLibrary|GetHTCPupilData))
  (bind _returnvalue_3 (Class|ViveOpenXREyeTrackerFunctionLibrary|GetHTCEyeGazeValidData))
  (bind _eyeinformationwidget (Variables|Default|GetEyeInformationWidget))
  (bind _eyeinformationwidget_2 (Variables|Default|GetEyeInformationWidget))
  (bind _eyeinformationwidget_3 (Variables|Default|GetEyeInformationWidget))
  (bind (_x _y) (Math|Vector2D|BreakVector2D (.lefteyepupilposition _returnvalue_2)))
  (bind (_x_2 _y_2) (Math|Vector2D|BreakVector2D (.righteyepupilposition _returnvalue_2)))
  (bind _outgazedata (Class|EyeTrackerFunctionLibrary|GetStereoGazeData))
  (Rendering|Components|TextRender|SetText (Variables|/Game/LibrarySamples/VIVE/EyeTracking/Blueprints/WBP_EyeInformation.WBP_EyeInformation_C|GetR_isVaild _eyeinformationwidget_2) (Utilities|Text|ToText(Boolean) (.righteyegazevalid _returnvalue_3)))
  (Rendering|Components|TextRender|SetText (Variables|/Game/LibrarySamples/VIVE/EyeTracking/Blueprints/WBP_EyeInformation.WBP_EyeInformation_C|GetL_isVaild _eyeinformationwidget_2) (Utilities|Text|ToText(Boolean) (.lefteyegazevalid _returnvalue_3)))
  (Rendering|Components|TextRender|SetText (Variables|/Game/LibrarySamples/VIVE/EyeTracking/Blueprints/WBP_EyeInformation.WBP_EyeInformation_C|GetR_poision _eyeinformationwidget_2) (Utilities|Text|ToText(String) (.righteyeorigin _outgazedata)))
  (Rendering|Components|TextRender|SetText (Variables|/Game/LibrarySamples/VIVE/EyeTracking/Blueprints/WBP_EyeInformation.WBP_EyeInformation_C|GetL_poision _eyeinformationwidget_2) (Utilities|Text|ToText(String) (.lefteyeorigin _outgazedata)))
  (Rendering|Components|TextRender|SetText (Variables|/Game/LibrarySamples/VIVE/EyeTracking/Blueprints/WBP_EyeInformation.WBP_EyeInformation_C|GetR_direction _eyeinformationwidget_2) (Utilities|Text|ToText(String) (.righteyedirection _outgazedata)))
  (Rendering|Components|TextRender|SetText (Variables|/Game/LibrarySamples/VIVE/EyeTracking/Blueprints/WBP_EyeInformation.WBP_EyeInformation_C|GetL_direction _eyeinformationwidget_2) (Utilities|Text|ToText(String) (.lefteyedirection _outgazedata)))
  (Rendering|Components|TextRender|SetText (Variables|/Game/LibrarySamples/VIVE/EyeTracking/Blueprints/WBP_EyeInformation.WBP_EyeInformation_C|GetR_isDiameterValid _eyeinformationwidget_3) (Utilities|Text|ToText(Boolean) (.righteyediametervalid _returnvalue_2)))
  (Rendering|Components|TextRender|SetText (Variables|/Game/LibrarySamples/VIVE/EyeTracking/Blueprints/WBP_EyeInformation.WBP_EyeInformation_C|GetL_isDiameterValid _eyeinformationwidget_3) (Utilities|Text|ToText(Boolean) (.lefteyediametervalid _returnvalue_2)))
  (Rendering|Components|TextRender|SetText (Variables|/Game/LibrarySamples/VIVE/EyeTracking/Blueprints/WBP_EyeInformation.WBP_EyeInformation_C|GetR_isEyePoistionValid _eyeinformationwidget_3) (Utilities|Text|ToText(Boolean) (.righteyepositionvalid _returnvalue_2)))
  (Rendering|Components|TextRender|SetText (Variables|/Game/LibrarySamples/VIVE/EyeTracking/Blueprints/WBP_EyeInformation.WBP_EyeInformation_C|GetL_isEyePoistionValid _eyeinformationwidget_3) (Utilities|Text|ToText(Boolean) (.lefteyepositionvalid _returnvalue_2)))
  (Rendering|Components|TextRender|SetText (Variables|/Game/LibrarySamples/VIVE/EyeTracking/Blueprints/WBP_EyeInformation.WBP_EyeInformation_C|GetR_pupilDiameter _eyeinformationwidget_3) (Utilities|Text|ToText(Float) (.righteyepupildiameter _returnvalue_2) "HalfToEven"))
  (Rendering|Components|TextRender|SetText (Variables|/Game/LibrarySamples/VIVE/EyeTracking/Blueprints/WBP_EyeInformation.WBP_EyeInformation_C|GetL_pupilDiameter _eyeinformationwidget_3) (Utilities|Text|ToText(Float) (.lefteyepupildiameter _returnvalue_2) "HalfToEven"))
  (Rendering|Components|TextRender|SetText (Variables|/Game/LibrarySamples/VIVE/EyeTracking/Blueprints/WBP_EyeInformation.WBP_EyeInformation_C|GetR_pupilPoision _eyeinformationwidget_3) (Utilities|Text|ToText(String) (Utilities|String|Append (Utilities|String|ToString(Float) _x_2) ", " (Utilities|String|ToString(Float) _y_2))))
  (Rendering|Components|TextRender|SetText (Variables|/Game/LibrarySamples/VIVE/EyeTracking/Blueprints/WBP_EyeInformation.WBP_EyeInformation_C|GetL_pupilPoision _eyeinformationwidget_3) (Utilities|Text|ToText(String) (Utilities|String|Append (Utilities|String|ToString(Float) _x) ", " (Utilities|String|ToString(Float) _y))))
  (Rendering|Components|TextRender|SetText (Variables|/Game/LibrarySamples/VIVE/EyeTracking/Blueprints/WBP_EyeInformation.WBP_EyeInformation_C|GetR_isGemoetricValid _eyeinformationwidget) (Utilities|Text|ToText(Boolean) (.righteyeisvalid _returnvalue)))
  (Rendering|Components|TextRender|SetText (Variables|/Game/LibrarySamples/VIVE/EyeTracking/Blueprints/WBP_EyeInformation.WBP_EyeInformation_C|GetL_isGemoetricValid _eyeinformationwidget) (Utilities|Text|ToText(Boolean) (.lefteyeisvalid _returnvalue)))
  (Rendering|Components|TextRender|SetText (Variables|/Game/LibrarySamples/VIVE/EyeTracking/Blueprints/WBP_EyeInformation.WBP_EyeInformation_C|GetR_Openness _eyeinformationwidget) (Utilities|Text|ToText(Float) (.righteyeopenness _returnvalue) "HalfToEven"))
  (Rendering|Components|TextRender|SetText (Variables|/Game/LibrarySamples/VIVE/EyeTracking/Blueprints/WBP_EyeInformation.WBP_EyeInformation_C|GetL_Openness _eyeinformationwidget) (Utilities|Text|ToText(Float) (.lefteyeopenness _returnvalue) "HalfToEven"))
  (Rendering|Components|TextRender|SetText (Variables|/Game/LibrarySamples/VIVE/EyeTracking/Blueprints/WBP_EyeInformation.WBP_EyeInformation_C|GetR_Wide _eyeinformationwidget) (Utilities|Text|ToText(Float) (.righteyewide _returnvalue) "HalfToEven"))
  (Rendering|Components|TextRender|SetText (Variables|/Game/LibrarySamples/VIVE/EyeTracking/Blueprints/WBP_EyeInformation.WBP_EyeInformation_C|GetL_Wide _eyeinformationwidget) (Utilities|Text|ToText(Float) (.lefteyewide _returnvalue) "HalfToEven"))
  (Rendering|Components|TextRender|SetText (Variables|/Game/LibrarySamples/VIVE/EyeTracking/Blueprints/WBP_EyeInformation.WBP_EyeInformation_C|GetR_Squeeze _eyeinformationwidget) (Utilities|Text|ToText(Float) (.righteyesqueeze _returnvalue) "HalfToEven"))
  (Rendering|Components|TextRender|SetText (Variables|/Game/LibrarySamples/VIVE/EyeTracking/Blueprints/WBP_EyeInformation.WBP_EyeInformation_C|GetL_Squeeze _eyeinformationwidget) (Utilities|Text|ToText(Float) (.lefteyesqueeze _returnvalue) "HalfToEven")))

(fn ConstructionScript)