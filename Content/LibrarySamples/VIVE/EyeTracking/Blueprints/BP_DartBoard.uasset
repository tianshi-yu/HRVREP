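; VIVE eye-tracking sample dart board that shows where the user is looking through a dynamic material.
; Each tick it line-traces stereo per-eye gaze, falling back to combined gaze, to find the focus point.
; Distance and signed angle from the board center give ring (bend) and sector (pie) indices for the material.
; The board aligns to camera height and yaw shortly after start and again on Z.
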(event EventTick
  (params (DeltaSeconds :type Float%20%28single-precision%29))
  (bind _returnvalue (Game|GetPlayerCameraManager 0))
  (bind _returnvalue_2 (Game|GetPlayerCameraManager 0))
  (bind _returnvalue_3 (Transformation|GetActorLocation))
  (bind _matinst (Variables|Default|GetMatInst))
  (bind _originallocation (Variables|Default|GetOriginalLocation))
  (bind _returnvalue_4 (Camera|GetCameraLocation _returnvalue))
  (bind _array (Utilities|Array|MakeArray _returnvalue_2))
  (bind _returnvalue_5 (Math|Rotator|FindLookatRotation _returnvalue_3 _returnvalue_4))
  (bind (_roll _pitch _yaw) (Math|Rotator|BreakRotator _returnvalue_5))
  (bind (_outgazedata _returnvalue_6) (Class|EyeTrackerFunctionLibrary|GetStereoGazeData))
  (Variables|Default|SetOut%20Stereo%20Gaze%20Data _outgazedata)
  (if (not _returnvalue_6)
    (bind (_outgazedata_2 _returnvalue_7) (Class|EyeTrackerFunctionLibrary|GetGazeData))
    (Variables|Default|SetOut%20Gaze%20Data _outgazedata_2)
    (Utilities|FlowControl|Sequence
      (:then_0
        (if (not (Variables|Default|GetAlreadyMoveDart)) :!label _label
          (Utilities|FlowControl|Delay 0.5)
          ;[1 1 1] Set dart board location and rotation
          (Utilities|FlowControl|Sequence
            (:then_0
              (Transformation|SetActorLocation (Math|Vector|MakeVector (.x _originallocation) (.y _originallocation) (.z (Camera|GetCameraLocation _returnvalue))) false false)
              (Transformation|SetActorRotation (Math|Rotator|MakeRotator _roll 0.0 (+ _yaw 1.8e+02))))
            (:then_1
              (Variables|Default|SetAlreadyMoveDart true)))))
      (:then_1
        ;[1 1 1] Use gaze date to line trace
        (if _returnvalue_7
          (bind (_outhit _returnvalue_8) (Collision|LineTraceByChannel (.gazeorigin (Variables|Default|GetOut%20Gaze%20Data)) (+ (.gazeorigin (Variables|Default|GetOut%20Gaze%20Data)) (* (.gazedirection (Variables|Default|GetOut%20Gaze%20Data)) 1e+03)) "TraceTypeQuery1" true (Utilities|Array|MakeArray (Game|GetPlayerCameraManager 0)) "ForOneFrame" false "(R=1.000000,G=0.000000,B=0.000000,A=1.000000)" "(R=0.000000,G=1.000000,B=0.000000,A=1.000000)" 0.1))
          (if _returnvalue_8
            (Variables|Default|SetFocusPos (.Location (Collision|BreakHitResult _outhit)))
            ;[1 1 1] Update dart board material
            (Rendering|Material|SetVectorParameterValue _matinst "MeshCenter" (Math|Conversions|ToLinearColor(Vector) (Transformation|GetActorLocation)) :!class /Script/Engine.MaterialInstanceDynamic :!label _label_2)
            (Rendering|Material|SetVectorParameterValue _matinst "MeshForward" (Math|Conversions|ToLinearColor(Vector) (Transformation|GetActorForwardVector)) :!class /Script/Engine.MaterialInstanceDynamic)
            (Rendering|Material|SetVectorParameterValue _matinst "MeshRight" (Math|Conversions|ToLinearColor(Vector) (Transformation|GetActorRightVector)) :!class /Script/Engine.MaterialInstanceDynamic)
            (Rendering|Material|SetScalarParameterValue _matinst "BendIndex" (Math|Conversions|ToFloat(Integer) (Utilities|CalculateBendIndex)) :!class /Script/Engine.MaterialInstanceDynamic)
            (Rendering|Material|SetScalarParameterValue _matinst "PieIndex" (Math|Conversions|ToFloat(Integer) (Utilities|CalculatePieIndex)) :!class /Script/Engine.MaterialInstanceDynamic)
            (Rendering|Material|SetScalarParameterValue _matinst "Scale" (.y (Transformation|GetActorScale3D)) :!class /Script/Engine.MaterialInstanceDynamic)))))
    (else
      (Utilities|FlowControl|Sequence
        (:then_0
          (goto _label))
        (:then_1
          ;[1 1 1] Use stereo gaze date to line trace
          (bind (_outhit_2 _returnvalue_9) (Collision|LineTraceByChannel (.lefteyeorigin (Variables|Default|GetOut%20Stereo%20Gaze%20Data)) (+ (.lefteyeorigin (Variables|Default|GetOut%20Stereo%20Gaze%20Data)) (* (.lefteyedirection (Variables|Default|GetOut%20Stereo%20Gaze%20Data)) 1e+03)) "TraceTypeQuery1" true _array "ForOneFrame" false "(R=1.000000,G=0.000000,B=0.000000,A=1.000000)" "(R=0.000000,G=1.000000,B=0.000000,A=1.000000)" 0.1))
          (Variables|Default|SetFocusPos (.Location (Collision|BreakHitResult _outhit_2))))
        (:then_2
          (bind (_outhit_3 _returnvalue_10) (Collision|LineTraceByChannel (.righteyeorigin (Variables|Default|GetOut%20Stereo%20Gaze%20Data)) (+ (.righteyeorigin (Variables|Default|GetOut%20Stereo%20Gaze%20Data)) (* (.righteyedirection (Variables|Default|GetOut%20Stereo%20Gaze%20Data)) 1e+03)) "TraceTypeQuery1" true _array "ForOneFrame" false "(R=1.000000,G=0.000000,B=0.000000,A=1.000000)" "(R=0.000000,G=1.000000,B=0.000000,A=1.000000)" 0.1))
          (Variables|Default|SetFocusPos (.Location (Collision|BreakHitResult _outhit_3)))))
      (if (or _returnvalue_9 _returnvalue_10)
        (goto _label_2)))))

(event EventBeginPlay
  (bind _dartboard (Variables|Default|GetDartBoard))
  (bind _returnvalue (Rendering|Material|CreateDynamicMaterialInstance _dartboard 0 (Rendering|Material|GetMaterial _dartboard 0) "None" :!class /Script/Engine.PrimitiveComponent))
  (bind _output_get (Variables|Default|SetMatInst _returnvalue))
  (Rendering|Material|SetScalarParameterValue _output_get "BendCount" (Math|Conversions|ToFloat(Integer) (Variables|BoardParameters|GetBendCount)) :!class /Script/Engine.MaterialInstanceDynamic)
  (Rendering|Material|SetScalarParameterValue _output_get "PieCount" (Math|Conversions|ToFloat(Integer) (Variables|BoardParameters|GetPieCount)) :!class /Script/Engine.MaterialInstanceDynamic)
  (Rendering|Material|SetScalarParameterValue _output_get "FrameWidth" (Math|Conversions|ToFloat(Integer) (Variables|BoardParameters|GetFrameWidth)) :!class /Script/Engine.MaterialInstanceDynamic)
  (Variables|Default|SetOriginalLocation (Transformation|GetActorLocation))
  (Input|EnableInput (Game|GetPlayerController 0)))

(event Input|KeyboardEvents|Z
  (params (Key :type Key%20Structure))
  (bind _returnvalue (Game|GetPlayerCameraManager 0))
  (bind _returnvalue_2 (Transformation|GetActorLocation))
  (bind _originallocation (Variables|Default|GetOriginalLocation))
  (bind _returnvalue_3 (Camera|GetCameraLocation _returnvalue))
  (bind _returnvalue_4 (Math|Rotator|FindLookatRotation _returnvalue_2 _returnvalue_3))
  (bind (_roll _pitch _yaw) (Math|Rotator|BreakRotator _returnvalue_4))
  (:Pressed
    ;[1 1 1] Set dart board location and rotation
    (Transformation|SetActorLocation (Math|Vector|MakeVector (.x _originallocation) (.y _originallocation) (.z (Camera|GetCameraLocation _returnvalue))) false false)
    (Transformation|SetActorRotation (Math|Rotator|MakeRotator _roll 0.0 (+ _yaw 1.8e+02)))))

(fn ConstructionScript)