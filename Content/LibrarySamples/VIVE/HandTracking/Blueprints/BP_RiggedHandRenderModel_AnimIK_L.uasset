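; BP_RiggedHandRenderModel_AnimIK_L is the left-hand variant of a rigged hand render model in the VIVE hand tracking sample.
; It casts the hand skeletal mesh's anim instance to ABP_LeftHand and caches it.
; Its events forward per-bone goal positions with alpha, and joint rotations keyed by hand keypoint, to that AnimBP, leaving posing to the animation side.
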(event EventSetupAnimBPInst
  (bind _asabp_left_hand (Utilities|Casting|CastToABP_LeftHand (Components|SkeletalMesh|GetAnimInstance (Variables|Default|GetSkeletalMesh_Hand))))
  (Variables|Default|SetLeft%20Hand%20Anim%20Blueprint _asabp_left_hand))

(event EventUpdateAnimBPGoalPosition
  (params (BoneName :type Name :default "None") (Goal%20Position :type Vector :default "0, 0, 0") (Goal%20Position%20Alpha :type Float%20%28double-precision%29))
  (Default|UpdateGoalPosition (Variables|Default|GetLeft%20Hand%20Anim%20Blueprint) BoneName Goal%20Position Goal%20Position%20Alpha))

(event EventUpdateAnimBPJointRotation
  (params (EHandKeypoint :type EHandKeypoint%20Enum :default "Palm") (InRotation :type Rotator :default "0, 0, 0"))
  (Default|SetBoneRotationbyEHandKeypoint (Variables|Default|GetLeft%20Hand%20Anim%20Blueprint) EHandKeypoint InRotation))

(fn ConstructionScript
  (|CallParentFunction))