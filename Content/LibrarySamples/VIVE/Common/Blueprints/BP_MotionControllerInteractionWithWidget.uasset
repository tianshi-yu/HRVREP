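; Motion controller laser pointer actor that attaches to the player pawn's controller matching MotionSource to interact with widgets.
; Each tick it line traces from Aim, moves a HitPoint marker and fires OnHitActor when the hit actor changes.
; The WidgetInteraction component shows while the controller is tracked or AlwaysShow is set.
; Trigger input past a threshold presses a simulated pointer key, with paired DoOnce gates governing press and release.
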(event Custom|Completed
  (bind _simulatedkey (Variables|Default|GetSimulatedKey))
  (bind _widgetinteraction (Variables|Default|GetWidgetInteraction))
  (Utilities|FlowControl|DoOnce false
    (:Completed
      (Class|WidgetInteractionComponent|ReleasePointerKey _widgetinteraction _simulatedkey)
      (Utilities|FlowControl|DoOnce false) ; enters at Reset
    )))

(event Custom|InteractionTrigger
  (params (ActionValue :type Float%20%28double-precision%29))
  (bind _simulatedkey (Variables|Default|GetSimulatedKey))
  (bind _widgetinteraction (Variables|Default|GetWidgetInteraction))
  (if (>= ActionValue 0.7)
    (Utilities|FlowControl|DoOnce false
      (:Completed
        (Class|WidgetInteractionComponent|PressPointerKey _widgetinteraction _simulatedkey)
        (Utilities|FlowControl|DoOnce false) ; enters at Reset
      ))))

(event EventBeginPlay
  (Rendering|SetVisibility (Variables|Default|GetWidgetInteraction) false true)
  (bind _returnvalue (CallFunction|AttachtoPawnMotionController))
  (Actor|Tick|SetActorTickEnabled _returnvalue)
  (if _returnvalue
    (Transformation|SetRelativeScale3D (Variables|Default|GetHitPoint) (Math|Conversions|ToVector(Float) (/ (Variables|Default|GetTraceEnd) 1e+03)))
    (else
      (Development|PrintString (Utilities|String|Append "Motion Controller [" (Utilities|String|ToString(Name) (Variables|Default|GetMotionSource)) "] not found")))))

(event Collision|EventActorBeginOverlap
  (params (OtherActor :type Actor%20Object%20Reference)))

(event EventTick
  (params (DeltaSeconds :type Float%20%28single-precision%29))
  (bind _hitpoint (Variables|Default|GetHitPoint))
  (bind _aim (Variables|Default|GetAim))
  (bind _returnvalue (Transformation|GetWorldLocation _aim))
  (Utilities|FlowControl|Sequence
    (:then_0
      (bind (_outhit _returnvalue_2) (Collision|LineTraceByChannel _returnvalue (+ _returnvalue (* (Math|Vector|GetForwardVector _aim) (Variables|Default|GetTraceEnd))) "TraceTypeQuery1" false (Variables|Default|GetActors%20to%20Ignore) "None" true "(R=1.000000,G=0.000000,B=0.000000,A=1.000000)" "(R=0.000000,G=1.000000,B=0.000000,A=1.000000)" 1.0))
      (if (!= (Variables|Default|GetHitActor) (.HitActor (Collision|BreakHitResult _outhit)))
        (Default|CallOnHitActor (.HitActor (Collision|BreakHitResult _outhit))))
      (if _returnvalue_2
        (Transformation|SetWorldLocation _hitpoint (.Location (Collision|BreakHitResult _outhit)) false true)
        (Variables|Default|SetHitActor (.HitActor (Collision|BreakHitResult _outhit)))
        (else
          (Transformation|SetWorldLocation _hitpoint (.TraceEnd (Collision|BreakHitResult _outhit)) false true)
          (Variables|Default|SetHitActor 0))))
    (:then_1
      ;[1 1 1] Set Visibility
      (if (Variables|Default|GetAlwaysShow)
        (Utilities|FlowControl|Sequence :!label _label
          (:then_0
            (if (not (Rendering|IsVisible (Variables|Default|GetWidgetInteraction)))
              (Rendering|SetVisibility (Variables|Default|GetWidgetInteraction) true true))))
        (elif (Class|MotionControllerComponent|IsTracked (Variables|Default|GetMotionController))
          (goto _label)
          (elif (Rendering|IsVisible (Variables|Default|GetWidgetInteraction))
            (Rendering|SetVisibility (Variables|Default|GetWidgetInteraction) false true)))))))

(fn ConstructionScript)

(fn AttachtoPawnMotionController
  (for _array_element (Actor|GetComponentsByClass (Game|Player|GetPlayerPawn 0) "/Script/HeadMountedDisplay.MotionControllerComponent")
    (Variables|Default|SetMotionController _array_element)
    (if (== (Variables|/Script/HeadMountedDisplay.MotionControllerComponent|GetMotionSource _array_element) (Variables|Default|GetMotionSource))
      (bind _returnvalue (Transformation|AttachComponentToComponent _array_element "None" "KeepWorld" "KeepWorld" "KeepWorld" true))
      (return _returnvalue)))
  (return false))