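; Sample board actor that shows VIVE OpenXR display refresh rate and live FPS on a widget component.
; On BeginPlay it caches the widget and binds to the refresh rate change notification, which writes the previous, new and queried current rates into its text fields.
; Tick smooths FPS from delta time with a frame-time-weighted lerp and pushes it to the widget every frame.
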(event Custom|DisplayRefreshRateChangedDelegate_Event
  (params (FromDisplayRefreshRate :type Float%20%28single-precision%29) (ToDisplayRefreshRate :type Float%20%28single-precision%29))
  (bind (_outdisplayrefreshrate _returnvalue) (Class|ViveOpenXRDisplayRefreshRateFunctionLibrary|GetDisplayRefreshRate))
  (bind _refreshratewidget (Variables|Default|GetRefreshRateWidget))
  ;[1 1 1] Listen Refresh Rate change event and set values to Widget Object for updating value
  (Variables|/Script/UMG.TextBlock|SetText (Variables|/Game/LibrarySamples/VIVE/DisplayRefreshRate/Blueprints/BP_DisplayRefreshRateWidget.BP_DisplayRefreshRateWidget_C|GetSwitchFrom_Text _refreshratewidget) (Utilities|Text|ToText(Float) FromDisplayRefreshRate "HalfToEven"))
  (Variables|/Script/UMG.TextBlock|SetText (Variables|/Game/LibrarySamples/VIVE/DisplayRefreshRate/Blueprints/BP_DisplayRefreshRateWidget.BP_DisplayRefreshRateWidget_C|GetSwitchTo_Text _refreshratewidget) (Utilities|Text|ToText(Float) ToDisplayRefreshRate "HalfToEven"))
  ;[1 1 1] UpdateCurrentRefreshRate
  (if _returnvalue
    (Variables|/Script/UMG.TextBlock|SetText (Variables|/Game/LibrarySamples/VIVE/DisplayRefreshRate/Blueprints/BP_DisplayRefreshRateWidget.BP_DisplayRefreshRateWidget_C|GetCurrentRefreshRate_Text _refreshratewidget) (Utilities|Text|ToText(Float) _outdisplayrefreshrate "HalfToEven"))))

(event EventBeginPlay
  (Utilities|FlowControl|Sequence
    (:then_0
      ;[1 1 1] Get Widget Object Reference
      (bind _asbp_display_refresh_rate_widget (Utilities|Casting|CastToBP_DisplayRefreshRateWidget (UserInterface|GetUserWidgetObject (Variables|Default|GetWidget))))
      (Variables|Default|SetRefreshRateWidget _asbp_display_refresh_rate_widget))
    (:then_1
      ;[1 1 1] Listen Refresh Rate change event and set values to Widget Object for updating value
      (EventDispatchers|AssignDisplayRefreshRateChangedDelegate (Variables|Default|GetViveOpenXRNotifications) (delegate Custom|DisplayRefreshRateChangedDelegate_Event)))))

(event Collision|EventActorBeginOverlap
  (params (OtherActor :type Actor%20Object%20Reference)))

(event EventTick
  (params (DeltaSeconds :type Float%20%28single-precision%29))
  (Utilities|FlowControl|Sequence
    (:then_0
      ;[1 1 1] Apply lerp in FPS
      (if (== DeltaSeconds 0.0)
        (Variables|Default|SetFPS 0.0)
        (else
          (Variables|Default|SetFPS (Math|Float|Lerp (Variables|Default|GetFPS) (/ 1.0 DeltaSeconds) (/ DeltaSeconds (+ 0.5 DeltaSeconds)))))))
    (:then_1
      ;[1 1 1] Set FPS to Widget Object
      (Variables|/Script/UMG.TextBlock|SetText (Variables|/Game/LibrarySamples/VIVE/DisplayRefreshRate/Blueprints/BP_DisplayRefreshRateWidget.BP_DisplayRefreshRateWidget_C|GetFPS_Text (Variables|Default|GetRefreshRateWidget)) (Utilities|Text|ToText(Float) (Variables|Default|GetFPS) "HalfToEven")))))

(fn ConstructionScript)