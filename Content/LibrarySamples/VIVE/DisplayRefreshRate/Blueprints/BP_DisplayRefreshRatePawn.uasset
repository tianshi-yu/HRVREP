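; VR pawn for the VIVE display refresh rate sample that lets the player interact with widgets using the right controller trigger.
; On BeginPlay it sets a local-floor tracking origin, enables input and adds the VIVE Enhanced Input mapping context.
; Right trigger press and release are forwarded to its WidgetInteraction object, and Escape quits the game.
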(event Input|EnhancedActionEvents|EnhancedInputActionIA_Keys_TriggerClick_R
  (params (ActionValue :type Boolean) (ElapsedSeconds :type Float%20%28double-precision%29) (TriggeredSeconds :type Float%20%28double-precision%29) (InputAction :type Input%20Action%20Object%20Reference :default "/Game/2_BluePrints/2_AvatarSystemCore/EnhancedInput/IA_Keys/IA_Keys_TriggerClick_R.IA_Keys_TriggerClick_R"))
  (bind _widgetinteraction (Variables|Components|GetWidgetInteraction))
  (:Started
    (Default|InteractionTrigger _widgetinteraction 1.0))
  (:Completed
    (Default|Completed _widgetinteraction)))

(event EventBeginPlay
  (bind _returnvalue (Game|GetPlayerController 0))
  (Class|HeadMountedDisplayFunctionLibrary|SetTrackingOrigin "LocalFloor")
  (Input|EnableInput _returnvalue)
  (Input|AddMappingContext (PlayerController|LocalPlayerSubsystems|GetEnhancedInputLocalPlayerSubsystem _returnvalue) "/Game/2_BluePrints/2_AvatarSystemCore/EnhancedInput/IMC_VIVEInputs.IMC_VIVEInputs" 0 "(bIgnoreAllPressedKeysUntilRelease=True,bForceImmediately=False,bNotifyUserSettings=False)"))

(event Input|KeyboardEvents|Escape
  (params (Key :type Key%20Structure))
  (:Pressed
    (Game|QuitGame 0 "Quit" false)))

(fn ConstructionScript)