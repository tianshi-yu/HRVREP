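; Hand-attached interactor from the VIVE display refresh rate sample that aims a laser at UI widgets and clicks them.
; On Tick it spawns a beam particle once, then aligns it with the widget interaction component whenever AlwaysShow is set or the hand's motion controller data is valid.
; Enhanced Input drives pointer key press and release from a thresholded trigger value, with DoOnce gates preventing repeats.
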(event Custom|Completed
  (bind _simulatedkey (Variables|Default|GetSimulatedKey))
  (bind _widgetinteraction_r (Variables|Default|GetWidgetInteraction_R))
  (Utilities|FlowControl|DoOnce false
    (:Completed
      (Class|WidgetInteractionComponent|ReleasePointerKey _widgetinteraction_r _simulatedkey)
      (Utilities|FlowControl|DoOnce false) ; enters at Reset
    )))

(event Custom|InteractionTrigger
  (params (ActionValue :type Float%20%28double-precision%29))
  (bind _simulatedkey (Variables|Default|GetSimulatedKey))
  (bind _widgetinteraction_r (Variables|Default|GetWidgetInteraction_R))
  (if (>= ActionValue 0.7)
    (Utilities|FlowControl|DoOnce false
      (:Completed
        (Class|WidgetInteractionComponent|PressPointerKey _widgetinteraction_r _simulatedkey)
        (Utilities|FlowControl|DoOnce false) ; enters at Reset
      ))))

(event EventBeginPlay
  (Rendering|SetVisibility (Variables|Default|GetWidgetInteraction_R) false true)
  (Input|AddMappingContext (PlayerController|LocalPlayerSubsystems|GetEnhancedInputLocalPlayerSubsystem (Game|GetPlayerController 0)) "/Game/2_BluePrints/2_AvatarSystemCore/EnhancedInput/IMC_VIVEInputs.IMC_VIVEInputs" 0 "(bIgnoreAllPressedKeysUntilRelease=True,bForceImmediately=False,bNotifyUserSettings=False)"))

(event Collision|EventActorBeginOverlap
  (params (OtherActor :type Actor%20Object%20Reference)))

(event EventTick
  (params (DeltaSeconds :type Float%20%28single-precision%29))
  (bind _widgetinteraction_r (Variables|Default|GetWidgetInteraction_R))
  (bind _returnvalue (Transformation|GetWorldLocation _widgetinteraction_r))
  (Utilities|FlowControl|Sequence
    (:then_0
      ;[1 1 1] Spawn Beam
      (Utilities|FlowControl|DoOnce false
        (:Completed
          (bind _returnvalue_2 (Effects|SpawnEmitterAttached "/Game/LibrarySamples/VIVE/DisplayRefreshRate/Material/P_LaserSystemForBeam.P_LaserSystemForBeam" (Variables|Default|GetWidgetInteraction_R) "None"))
          (bind _output_get (Variables|Default|SetLaser%20Particle_R _returnvalue_2))
          (Rendering|SetVisibility _output_get (Variables|Default|GetAlwaysShow) true))))
    (:then_1
      ;[1 1 1] Set Visibility
      (if (Variables|Default|GetAlwaysShow)
        (Utilities|FlowControl|Sequence :!label _label
          (:then_0
            (if (not (Rendering|IsVisible (Variables|Default|GetWidgetInteraction_R)))
              (Rendering|SetVisibility (Variables|Default|GetWidgetInteraction_R) true true)))
          (:then_1
            ;[1 1 1] Get HandInteraction Aim pose to set up beam and select value to choose buttons.
            (Class|ParticleSystemComponent|SetBeamSourcePoint (Variables|Default|GetLaser%20Particle_R) 0 _returnvalue)
            (Class|ParticleSystemComponent|SetBeamEndPoint (Variables|Default|GetLaser%20Particle_R) 0 (+ _returnvalue (* (Math|Vector|GetForwardVector _widgetinteraction_r) 2e+03)))))
        (else
          (bind _motioncontrollerdata (Class|HeadMountedDisplayFunctionLibrary|GetMotionControllerData 0 (Variables|Default|GetHand)))
          (if (.bvalid _motioncontrollerdata)
            (goto _label)
            (elif (Rendering|IsVisible (Variables|Default|GetWidgetInteraction_R))
              (Rendering|SetVisibility (Variables|Default|GetWidgetInteraction_R) false true))))))))

(fn ConstructionScript)