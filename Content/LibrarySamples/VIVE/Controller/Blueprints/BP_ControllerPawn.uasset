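; VR pawn for the VIVE controller sample that tracks and displays both hand controllers, using a local-floor origin.
; Each tick reads motion controller data per hand and moves grip and aim pose components to match.
; Once a device name appears, a DoOnce picks Cosmos or Focus 3 motion source and display mesh; the left hand tests the right device's name.
; Escape quits the game.
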(event EventBeginPlay
  (Class|HeadMountedDisplayFunctionLibrary|SetTrackingOrigin "LocalFloor"))

(event EventTick
  (params (DeltaSeconds :type Float%20%28single-precision%29))
  (bind _rightaimpose (Variables|Default|GetRightAimPose))
  (bind _rightgrippose (Variables|Default|GetRightGripPose))
  (bind _leftaimpose (Variables|Default|GetLeftAimPose))
  (bind _leftgrippose (Variables|Default|GetLeftGripPose))
  (Utilities|FlowControl|Sequence
    (:then_0
      (bind _motioncontrollerdata (Class|HeadMountedDisplayFunctionLibrary|GetMotionControllerData 0 "Right"))
      (bind _output_get (Variables|Default|SetDevice%20Name_R (.DeviceName (Utilities|Struct|BreakXRMotionControllerData _motioncontrollerdata))))
      (if (!= _output_get "")
        (Utilities|FlowControl|Sequence
          (:then_0
            (Utilities|FlowControl|DoOnce false
              (:Completed
                (if (== (Utilities|String|FindSubstring (Utilities|String|ToString(Name) (Variables|Default|GetDevice%20Name_R)) (Variables|Default|GetCosmos%20Name)) 0)
                  (Utilities|FlowControl|Sequence
                    (:then_0
                      (Variables|/Script/HeadMountedDisplay.MotionControllerComponent|SetMotionSource (Variables|Default|GetMotionController_R) "Right"))
                    (:then_1
                      (Variables|/Script/XRBase.XRDeviceVisualizationComponent|SetCustomDisplayMesh (Variables|Default|GetXRDeviceVisualization_R) (Variables|Model|GetCosmos%20model_R))))
                  (else
                    (Utilities|FlowControl|Sequence
                      (:then_0
                        (Variables|/Script/HeadMountedDisplay.MotionControllerComponent|SetMotionSource (Variables|Default|GetMotionController_R) "RightAim"))
                      (:then_1
                        (Variables|/Script/XRBase.XRDeviceVisualizationComponent|SetCustomDisplayMesh (Variables|Default|GetXRDeviceVisualization_R) (Variables|Model|GetFocus3%20model_R)))))))))
          (:then_1
            (Transformation|SetWorldLocation _rightgrippose (.GripPosition (Utilities|Struct|BreakXRMotionControllerData _motioncontrollerdata)) false false)
            (Transformation|SetWorldRotation _rightgrippose (Class|KismetMathLibrary|QuatRotator (.GripRotation (Utilities|Struct|BreakXRMotionControllerData _motioncontrollerdata))) false false)
            (Transformation|SetWorldLocation _rightaimpose (.AimPosition (Utilities|Struct|BreakXRMotionControllerData _motioncontrollerdata)) false false)
            (Transformation|SetWorldRotation _rightaimpose (Class|KismetMathLibrary|QuatRotator (.AimRotation (Utilities|Struct|BreakXRMotionControllerData _motioncontrollerdata))) false false)))))
    (:then_1
      (bind _motioncontrollerdata_2 (Class|HeadMountedDisplayFunctionLibrary|GetMotionControllerData 0 "Left"))
      (bind _output_get_2 (Variables|Default|SetDevice%20Name_L (.DeviceName (Utilities|Struct|BreakXRMotionControllerData _motioncontrollerdata_2))))
      (if (!= _output_get_2 "")
        (Utilities|FlowControl|Sequence
          (:then_0
            (Utilities|FlowControl|DoOnce false
              (:Completed
                (if (== (Utilities|String|FindSubstring (Utilities|String|ToString(Name) (Variables|Default|GetDevice%20Name_R)) (Variables|Default|GetCosmos%20Name)) 0)
                  (Utilities|FlowControl|Sequence
                    (:then_0
                      (Variables|/Script/HeadMountedDisplay.MotionControllerComponent|SetMotionSource (Variables|Default|GetMotionController_L) "Left"))
                    (:then_1
                      (Variables|/Script/XRBase.XRDeviceVisualizationComponent|SetCustomDisplayMesh (Variables|Default|GetXRDeviceVisualization_L) (Variables|Model|GetCosmos%20model_L))))
                  (else
                    (Utilities|FlowControl|Sequence
                      (:then_0
                        (Variables|/Script/HeadMountedDisplay.MotionControllerComponent|SetMotionSource (Variables|Default|GetMotionController_L) "LeftAim"))
                      (:then_1
                        (Variables|/Script/XRBase.XRDeviceVisualizationComponent|SetCustomDisplayMesh (Variables|Default|GetXRDeviceVisualization_L) (Variables|Model|GetFocus3%20model_L)))))))))
          (:then_1
            (Transformation|SetWorldLocation _leftgrippose (.GripPosition (Utilities|Struct|BreakXRMotionControllerData _motioncontrollerdata_2)) false false)
            (Transformation|SetWorldRotation _leftgrippose (Class|KismetMathLibrary|QuatRotator (.GripRotation (Utilities|Struct|BreakXRMotionControllerData _motioncontrollerdata_2))) false false)
            (Transformation|SetWorldLocation _leftaimpose (.AimPosition (Utilities|Struct|BreakXRMotionControllerData _motioncontrollerdata_2)) false false)
            (Transformation|SetWorldRotation _leftaimpose (Class|KismetMathLibrary|QuatRotator (.AimRotation (Utilities|Struct|BreakXRMotionControllerData _motioncontrollerdata_2))) false false)))))))

(event Input|KeyboardEvents|Escape
  (params (Key :type Key%20Structure))
  (:Pressed
    (Game|QuitGame 0 "Quit" false)))

(fn ConstructionScript)