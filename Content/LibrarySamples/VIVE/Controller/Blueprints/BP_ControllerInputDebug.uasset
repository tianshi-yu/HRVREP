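; Debug display actor for VIVE controller input, showing each hand's current key, trigger or grip axis, and thumbstick direction.
; When an HMD is enabled, BeginPlay sets floor tracking and adds the IMC_VIVEInputs mapping context.
; Enhanced Input events write key names to text renders and rotate color-tinted arrows with the thumbsticks.
; Tick prints trigger or grip axis per hand, chosen by flags from trigger/grip events, though right GripClick leaves its flag unchanged.
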(event Custom|LeftNotPressing
  (Rendering|Components|TextRender|SetText (Variables|Default|GetTextRender_DebugKeyLeft) (Utilities|Text|ToText(String) (Variables|Default|GetLeft%20Key))))

(event Custom|ShowRightAxisValue
  (params (Value :type Float%20%28single-precision%29))
  (Rendering|Components|TextRender|SetText (Variables|Default|GetTextRender_DebugAxisRight) (Utilities|Text|ToText(Float) Value "HalfToEven" false true 1 324 3)))

(event Custom|ShowLeftAxisValue
  (params (Value :type Float%20%28single-precision%29))
  (Rendering|Components|TextRender|SetText (Variables|Default|GetTextRender_DebugAxisLeft) (Utilities|Text|ToText(Float) Value "HalfToEven" false true 1 324 3)))

(event Custom|ShowDebugKeyRight
  (params (InKey :type String))
  (Rendering|Components|TextRender|SetText (Variables|Default|GetTextRender_DebugKeyRight) (Utilities|Text|ToText(String) (Utilities|String|Append (Variables|Default|GetRight%20Identifier) " " InKey))))

(event Custom|ShowDebugKeyLeft
  (params (InKey :type String))
  (Rendering|Components|TextRender|SetText (Variables|Default|GetTextRender_DebugKeyLeft) (Utilities|Text|ToText(String) (Utilities|String|Append (Variables|Default|GetLeft%20Identifier) " " InKey))))

(event Custom|RightNotPressing
  (Rendering|Components|TextRender|SetText (Variables|Default|GetTextRender_DebugKeyRight) (Utilities|Text|ToText(String) (Variables|Default|GetRight%20Key))))

(event Input|EnhancedActionEvents|EnhancedInputActionIA_Keys_TriggerTouch_R
  (params (ActionValue :type Boolean) (ElapsedSeconds :type Float%20%28double-precision%29) (TriggeredSeconds :type Float%20%28double-precision%29) (InputAction :type Input%20Action%20Object%20Reference :default "/Game/2_BluePrints/2_AvatarSystemCore/EnhancedInput/IA_Keys/IA_Keys_TriggerTouch_R.IA_Keys_TriggerTouch_R"))
  ;[1 1 1] TriggerTouch/GripTouch. These event will decide to show Axis of Trigger or Grip button.
  (:Started
    (CallFunction|ShowDebugKeyRight (Variables|KeyName|GetTrigger%20Touch))
    (Variables|Default|SetRightTrggerOrGrip true))
  (:Completed
    (CallFunction|RightNotPressing)))

(event Input|EnhancedActionEvents|EnhancedInputActionIA_Keys_Menu_L
  (params (ActionValue :type Boolean) (ElapsedSeconds :type Float%20%28double-precision%29) (TriggeredSeconds :type Float%20%28double-precision%29) (InputAction :type Input%20Action%20Object%20Reference :default "/Game/2_BluePrints/2_AvatarSystemCore/EnhancedInput/IA_Keys/IA_Keys_Menu_L.IA_Keys_Menu_L"))
  (:Triggered
    (CallFunction|ShowDebugKeyLeft (Variables|KeyName|GetMenu)))
  (:Completed
    (CallFunction|LeftNotPressing)))

(event Input|EnhancedActionEvents|EnhancedInputActionIA_Keys_GripClick_R
  (params (ActionValue :type Boolean) (ElapsedSeconds :type Float%20%28double-precision%29) (TriggeredSeconds :type Float%20%28double-precision%29) (InputAction :type Input%20Action%20Object%20Reference :default "/Game/2_BluePrints/2_AvatarSystemCore/EnhancedInput/IA_Keys/IA_Keys_GripClick_R.IA_Keys_GripClick_R"))
  (:Started
    (CallFunction|ShowDebugKeyRight (Variables|KeyName|GetGrip%20Click)))
  (:Completed
    (CallFunction|RightNotPressing)))

(event Input|EnhancedActionEvents|EnhancedInputActionIA_Keys_GripTouch_L
  (params (ActionValue :type Boolean) (ElapsedSeconds :type Float%20%28double-precision%29) (TriggeredSeconds :type Float%20%28double-precision%29) (InputAction :type Input%20Action%20Object%20Reference :default "/Game/2_BluePrints/2_AvatarSystemCore/EnhancedInput/IA_Keys/IA_Keys_GripTouch_L.IA_Keys_GripTouch_L"))
  ;[1 1 1] TriggerTouch/GripTouch. These event will decide to show Axis of Trigger or Grip button.
  (:Started
    (CallFunction|ShowDebugKeyLeft (Variables|KeyName|GetGrip%20Touch))
    (Variables|Default|SetLeftTrggerOrGrip false))
  (:Completed
    (CallFunction|LeftNotPressing)))

(event Input|EnhancedActionEvents|EnhancedInputActionIA_Keys_GripTouch_R
  (params (ActionValue :type Boolean) (ElapsedSeconds :type Float%20%28double-precision%29) (TriggeredSeconds :type Float%20%28double-precision%29) (InputAction :type Input%20Action%20Object%20Reference :default "/Game/2_BluePrints/2_AvatarSystemCore/EnhancedInput/IA_Keys/IA_Keys_GripTouch_R.IA_Keys_GripTouch_R"))
  ;[1 1 1] TriggerTouch/GripTouch. These event will decide to show Axis of Trigger or Grip button.
  (:Started
    (CallFunction|ShowDebugKeyRight (Variables|KeyName|GetGrip%20Touch))
    (Variables|Default|SetRightTrggerOrGrip false))
  (:Completed
    (CallFunction|RightNotPressing)))

(event Input|EnhancedActionEvents|EnhancedInputActionIA_Keys_Thumbstick_L
  (params (ActionValue :type Boolean) (ElapsedSeconds :type Float%20%28double-precision%29) (TriggeredSeconds :type Float%20%28double-precision%29) (InputAction :type Input%20Action%20Object%20Reference :default "/Game/2_BluePrints/2_AvatarSystemCore/EnhancedInput/IA_Keys/IA_Keys_Thumbstick_L.IA_Keys_Thumbstick_L"))
  (:Triggered
    (CallFunction|ShowDebugKeyLeft (Variables|KeyName|GetThumbStick)))
  (:Completed
    (CallFunction|LeftNotPressing)))

(event Input|EnhancedActionEvents|EnhancedInputActionIA_Keys_Thumbstick_R
  (params (ActionValue :type Boolean) (ElapsedSeconds :type Float%20%28double-precision%29) (TriggeredSeconds :type Float%20%28double-precision%29) (InputAction :type Input%20Action%20Object%20Reference :default "/Game/2_BluePrints/2_AvatarSystemCore/EnhancedInput/IA_Keys/IA_Keys_Thumbstick_R.IA_Keys_Thumbstick_R"))
  (:Triggered
    (CallFunction|ShowDebugKeyRight (Variables|KeyName|GetThumbStick)))
  (:Completed
    (CallFunction|RightNotPressing)))

(event Input|EnhancedActionEvents|EnhancedInputActionIA_Keys_ThumbstickTouch_L
  (params (ActionValue :type Boolean) (ElapsedSeconds :type Float%20%28double-precision%29) (TriggeredSeconds :type Float%20%28double-precision%29) (InputAction :type Input%20Action%20Object%20Reference :default "/Game/2_BluePrints/2_AvatarSystemCore/EnhancedInput/IA_Keys/IA_Keys_ThumbstickTouch_L.IA_Keys_ThumbstickTouch_L"))
  (:Triggered
    (CallFunction|ShowDebugKeyLeft (Variables|KeyName|GetThumbStick%20Touch)))
  (:Completed
    (CallFunction|LeftNotPressing)))

(event Input|EnhancedActionEvents|EnhancedInputActionIA_Keys_ThumbstickTouch_R
  (params (ActionValue :type Boolean) (ElapsedSeconds :type Float%20%28double-precision%29) (TriggeredSeconds :type Float%20%28double-precision%29) (InputAction :type Input%20Action%20Object%20Reference :default "/Game/2_BluePrints/2_AvatarSystemCore/EnhancedInput/IA_Keys/IA_Keys_ThumbstickTouch_R.IA_Keys_ThumbstickTouch_R"))
  (:Triggered
    (CallFunction|ShowDebugKeyRight (Variables|KeyName|GetThumbStick%20Touch)))
  (:Completed
    (CallFunction|RightNotPressing)))

(event Input|EnhancedActionEvents|EnhancedInputActionIA_Keys_ThumbstickX_L
  (params (ActionValue :type Float%20%28double-precision%29) (ElapsedSeconds :type Float%20%28double-precision%29) (TriggeredSeconds :type Float%20%28double-precision%29) (InputAction :type Input%20Action%20Object%20Reference :default "/Game/2_BluePrints/2_AvatarSystemCore/EnhancedInput/IA_Keys/IA_Keys_ThumbstickX_L.IA_Keys_ThumbstickX_L"))
  (Transformation|SetWorldRotation (Variables|Default|GetLeftArrow) (Math|Conversions|RotationFromXVector (Math|Vector|Normalize (Math|Vector|MakeVector (Input|EnhancedActionValues|GetIA_Keys_ThumbstickY_L) (Input|EnhancedActionValues|GetIA_Keys_ThumbstickX_L) 0.0))) false false))

(event Input|EnhancedActionEvents|EnhancedInputActionIA_Keys_ThumbstickX_R
  (params (ActionValue :type Float%20%28double-precision%29) (ElapsedSeconds :type Float%20%28double-precision%29) (TriggeredSeconds :type Float%20%28double-precision%29) (InputAction :type Input%20Action%20Object%20Reference :default "/Game/2_BluePrints/2_AvatarSystemCore/EnhancedInput/IA_Keys/IA_Keys_ThumbstickX_R.IA_Keys_ThumbstickX_R"))
  (Transformation|SetWorldRotation (Variables|Default|GetRightArrow) (Math|Conversions|RotationFromXVector (Math|Vector|Normalize (Math|Vector|MakeVector (Input|EnhancedActionValues|GetIA_Keys_ThumbstickY_R) (Input|EnhancedActionValues|GetIA_Keys_ThumbstickX_R) 0.0))) false false))

(event Input|EnhancedActionEvents|EnhancedInputActionIA_Keys_ThumbstickY_L
  (params (ActionValue :type Float%20%28double-precision%29) (ElapsedSeconds :type Float%20%28double-precision%29) (TriggeredSeconds :type Float%20%28double-precision%29) (InputAction :type Input%20Action%20Object%20Reference :default "/Game/2_BluePrints/2_AvatarSystemCore/EnhancedInput/IA_Keys/IA_Keys_ThumbstickY_L.IA_Keys_ThumbstickY_L"))
  (Transformation|SetWorldRotation (Variables|Default|GetLeftArrow) (Math|Conversions|RotationFromXVector (Math|Vector|Normalize (Math|Vector|MakeVector (Input|EnhancedActionValues|GetIA_Keys_ThumbstickY_L) (Input|EnhancedActionValues|GetIA_Keys_ThumbstickX_L) 0.0))) false false))

(event Input|EnhancedActionEvents|EnhancedInputActionIA_Keys_TriggerTouch_L
  (params (ActionValue :type Boolean) (ElapsedSeconds :type Float%20%28double-precision%29) (TriggeredSeconds :type Float%20%28double-precision%29) (InputAction :type Input%20Action%20Object%20Reference :default "/Game/2_BluePrints/2_AvatarSystemCore/EnhancedInput/IA_Keys/IA_Keys_TriggerTouch_L.IA_Keys_TriggerTouch_L"))
  ;[1 1 1] TriggerTouch/GripTouch. These event will decide to show Axis of Trigger or Grip button.
  (:Started
    (CallFunction|ShowDebugKeyLeft (Variables|KeyName|GetTrigger%20Touch))
    (Variables|Default|SetLeftTrggerOrGrip true))
  (:Completed
    (CallFunction|LeftNotPressing)))

(event Input|EnhancedActionEvents|EnhancedInputActionIA_Keys_ThumbstickY_R
  (params (ActionValue :type Float%20%28double-precision%29) (ElapsedSeconds :type Float%20%28double-precision%29) (TriggeredSeconds :type Float%20%28double-precision%29) (InputAction :type Input%20Action%20Object%20Reference :default "/Game/2_BluePrints/2_AvatarSystemCore/EnhancedInput/IA_Keys/IA_Keys_ThumbstickY_R.IA_Keys_ThumbstickY_R"))
  (Transformation|SetWorldRotation (Variables|Default|GetRightArrow) (Math|Conversions|RotationFromXVector (Math|Vector|Normalize (Math|Vector|MakeVector (Input|EnhancedActionValues|GetIA_Keys_ThumbstickY_R) (Input|EnhancedActionValues|GetIA_Keys_ThumbstickX_R) 0.0))) false false))

(event Input|EnhancedActionEvents|EnhancedInputActionIA_Keys_ThumbrestTouch_L
  (params (ActionValue :type Boolean) (ElapsedSeconds :type Float%20%28double-precision%29) (TriggeredSeconds :type Float%20%28double-precision%29) (InputAction :type Input%20Action%20Object%20Reference :default "/Game/2_BluePrints/2_AvatarSystemCore/EnhancedInput/IA_Keys/IA_Keys_ThumbrestTouch_L.IA_Keys_ThumbrestTouch_L"))
  (:Started
    (CallFunction|ShowDebugKeyLeft (Variables|KeyName|GetThumbRest)))
  (:Completed
    (CallFunction|LeftNotPressing)))

(event Input|EnhancedActionEvents|EnhancedInputActionIA_Keys_ThumbrestTouch_R
  (params (ActionValue :type Boolean) (ElapsedSeconds :type Float%20%28double-precision%29) (TriggeredSeconds :type Float%20%28double-precision%29) (InputAction :type Input%20Action%20Object%20Reference :default "/Game/2_BluePrints/2_AvatarSystemCore/EnhancedInput/IA_Keys/IA_Keys_ThumbrestTouch_R.IA_Keys_ThumbrestTouch_R"))
  (:Started
    (CallFunction|ShowDebugKeyRight (Variables|KeyName|GetThumbRest)))
  (:Completed
    (CallFunction|RightNotPressing)))

(event Input|EnhancedActionEvents|EnhancedInputActionIA_Keys_TriggerClick_L
  (params (ActionValue :type Boolean) (ElapsedSeconds :type Float%20%28double-precision%29) (TriggeredSeconds :type Float%20%28double-precision%29) (InputAction :type Input%20Action%20Object%20Reference :default "/Game/2_BluePrints/2_AvatarSystemCore/EnhancedInput/IA_Keys/IA_Keys_TriggerClick_L.IA_Keys_TriggerClick_L"))
  (:Started
    (CallFunction|ShowDebugKeyLeft (Variables|KeyName|GetTrigger%20Click))
    (Variables|Default|SetLeftTrggerOrGrip true))
  (:Completed
    (CallFunction|LeftNotPressing)))

(event Input|EnhancedActionEvents|EnhancedInputActionIA_Keys_TriggerClick_R
  (params (ActionValue :type Boolean) (ElapsedSeconds :type Float%20%28double-precision%29) (TriggeredSeconds :type Float%20%28double-precision%29) (InputAction :type Input%20Action%20Object%20Reference :default "/Game/2_BluePrints/2_AvatarSystemCore/EnhancedInput/IA_Keys/IA_Keys_TriggerClick_R.IA_Keys_TriggerClick_R"))
  (:Started
    (CallFunction|ShowDebugKeyRight (Variables|KeyName|GetTrigger%20Click))
    (Variables|Default|SetRightTrggerOrGrip true))
  (:Completed
    (CallFunction|RightNotPressing)))

(event Input|EnhancedActionEvents|EnhancedInputActionIA_Keys_APress_R
  (params (ActionValue :type Boolean) (ElapsedSeconds :type Float%20%28double-precision%29) (TriggeredSeconds :type Float%20%28double-precision%29) (InputAction :type Input%20Action%20Object%20Reference :default "/Game/2_BluePrints/2_AvatarSystemCore/EnhancedInput/IA_Keys/IA_Keys_APress_R.IA_Keys_APress_R"))
  (:Triggered
    (CallFunction|ShowDebugKeyRight (Variables|KeyName|GetA%20Press)))
  (:Completed
    (CallFunction|RightNotPressing)))

(event Input|EnhancedActionEvents|EnhancedInputActionIA_Keys_BPress_R
  (params (ActionValue :type Boolean) (ElapsedSeconds :type Float%20%28double-precision%29) (TriggeredSeconds :type Float%20%28double-precision%29) (InputAction :type Input%20Action%20Object%20Reference :default "/Game/2_BluePrints/2_AvatarSystemCore/EnhancedInput/IA_Keys/IA_Keys_BPress_R.IA_Keys_BPress_R"))
  (:Triggered
    (CallFunction|ShowDebugKeyRight (Variables|KeyName|GetB%20Press)))
  (:Completed
    (CallFunction|RightNotPressing)))

(event Input|EnhancedActionEvents|EnhancedInputActionIA_Keys_XPress_L
  (params (ActionValue :type Boolean) (ElapsedSeconds :type Float%20%28double-precision%29) (TriggeredSeconds :type Float%20%28double-precision%29) (InputAction :type Input%20Action%20Object%20Reference :default "/Game/2_BluePrints/2_AvatarSystemCore/EnhancedInput/IA_Keys/IA_Keys_XPress_L.IA_Keys_XPress_L"))
  (:Triggered
    (CallFunction|ShowDebugKeyLeft (Variables|KeyName|GetX%20Press)))
  (:Completed
    (CallFunction|LeftNotPressing)))

(event Input|EnhancedActionEvents|EnhancedInputActionIA_Keys_YPress_L
  (params (ActionValue :type Boolean) (ElapsedSeconds :type Float%20%28double-precision%29) (TriggeredSeconds :type Float%20%28double-precision%29) (InputAction :type Input%20Action%20Object%20Reference :default "/Game/2_BluePrints/2_AvatarSystemCore/EnhancedInput/IA_Keys/IA_Keys_YPress_L.IA_Keys_YPress_L"))
  (:Triggered
    (CallFunction|ShowDebugKeyLeft (Variables|KeyName|GetY%20Press)))
  (:Completed
    (CallFunction|LeftNotPressing)))

(event Input|EnhancedActionEvents|EnhancedInputActionIA_Keys_GripClick_L
  (params (ActionValue :type Boolean) (ElapsedSeconds :type Float%20%28double-precision%29) (TriggeredSeconds :type Float%20%28double-precision%29) (InputAction :type Input%20Action%20Object%20Reference :default "/Game/2_BluePrints/2_AvatarSystemCore/EnhancedInput/IA_Keys/IA_Keys_GripClick_L.IA_Keys_GripClick_L"))
  (:Started
    (CallFunction|ShowDebugKeyLeft (Variables|KeyName|GetGrip%20Click))
    (Variables|Default|SetLeftTrggerOrGrip false))
  (:Completed
    (CallFunction|LeftNotPressing)))

(event EventBeginPlay
  (bind _returnvalue (Game|GetPlayerController 0))
  (bind _rightarrow (Variables|Default|GetRightArrow))
  (bind _leftarrow (Variables|Default|GetLeftArrow))
  (Utilities|FlowControl|Sequence
    (:then_0
      (bind _returnvalue_2 (Rendering|Material|CreateDynamicMaterialInstance _rightarrow 0 (Rendering|Material|GetMaterial _rightarrow 0) "None" :!class /Script/Engine.PrimitiveComponent))
      (bind _output_get (Variables|Default|SetRightMatInst _returnvalue_2))
      (Rendering|Material|SetVectorParameterValue _output_get "Color" (Variables|Default|GetRightColor) :!class /Script/Engine.MaterialInstanceDynamic))
    (:then_1
      (bind _returnvalue_3 (Rendering|Material|CreateDynamicMaterialInstance _leftarrow 0 (Rendering|Material|GetMaterial _leftarrow 0) "None" :!class /Script/Engine.PrimitiveComponent))
      (bind _output_get_2 (Variables|Default|SetLeftMatInst _returnvalue_3))
      (Rendering|Material|SetVectorParameterValue _output_get_2 "Color" (Variables|Default|GetLeftColor) :!class /Script/Engine.MaterialInstanceDynamic))
    (:then_2
      (if (Class|HeadMountedDisplayFunctionLibrary|IsHeadMountedDisplayEnabled)
        (Class|HeadMountedDisplayFunctionLibrary|SetTrackingOrigin "LocalFloor")
        (Input|EnableInput _returnvalue)
        (Input|AddMappingContext (PlayerController|LocalPlayerSubsystems|GetEnhancedInputLocalPlayerSubsystem _returnvalue) "/Game/2_BluePrints/2_AvatarSystemCore/EnhancedInput/IMC_VIVEInputs.IMC_VIVEInputs" 0 "(bIgnoreAllPressedKeysUntilRelease=True,bForceImmediately=False,bNotifyUserSettings=False)")))))

(event EventTick
  (params (DeltaSeconds :type Float%20%28single-precision%29))
  ;[1 1 1] Update Trigger/Touch Axis
  (Utilities|FlowControl|Sequence
    (:then_0
      (if (Variables|Default|GetRightTrggerOrGrip)
        (CallFunction|ShowRightAxisValue (Input|EnhancedActionValues|GetIA_Keys_TriggerAxis_R))
        (else
          (CallFunction|ShowRightAxisValue (Input|EnhancedActionValues|GetIA_Keys_GripAxis_R)))))
    (:then_1
      (if (Variables|Default|GetLeftTrggerOrGrip)
        (CallFunction|ShowLeftAxisValue (Input|EnhancedActionValues|GetIA_Keys_TriggerAxis_L))
        (else
          (CallFunction|ShowLeftAxisValue (Input|EnhancedActionValues|GetIA_Keys_GripAxis_L)))))))

(fn ConstructionScript)